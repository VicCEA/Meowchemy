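; Player controller that opens the quest log and pause menu from Enhanced Input actions.
; Each action lazily creates its widget on first use, caches it, adds it to the viewport and switches input to UI-only with focus on that widget.
; The pause action also pauses the game; closing the menus and restoring input are not handled here.
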(event `EnhancedInput|/Game/Input/IA_ShowQuests`
  (params (ActionValue :type Boolean) (ElapsedSeconds :type "Float (double-precision)") (TriggeredSeconds :type "Float (double-precision)") (InputAction :type "InputAction Object Reference" :default "/Game/Input/IA_ShowQuests.IA_ShowQuests"))
  (:`Started`
    (`/Engine/EditorBlueprintResources/StandardMacros.IsValid` (`self.QuestMenu`)
      (:`Is Valid`
        _)
      (:`Is Not Valid`
        (bind _returnvalue (`|CreateWidget` "/Game/QuestSystem/Ui/W_QuestLog.W_QuestLog_C"))
        (set `self.QuestMenu` _returnvalue)))
    (`UserWidget.AddToViewport` (`self.QuestMenu`) 0)
    (`WidgetBlueprintLibrary.SetInputMode_UIOnlyEx` (`GameplayStatics.GetPlayerController` 0) (`self.QuestMenu`) "DoNotLock" true)))

(event `EnhancedInput|/Game/Input/IA_Pause`
  (params (ActionValue :type Boolean) (ElapsedSeconds :type "Float (double-precision)") (TriggeredSeconds :type "Float (double-precision)") (InputAction :type "InputAction Object Reference" :default "/Game/Input/IA_Pause.IA_Pause"))
  (:`Started`
    (`/Engine/EditorBlueprintResources/StandardMacros.IsValid` (`self.PauseMenu`)
      (:`Is Valid`
        _)
      (:`Is Not Valid`
        (bind _returnvalue (`|CreateWidget` "/Game/UI/WI_PauseMenu.WI_PauseMenu_C"))
        (set `self.PauseMenu` _returnvalue)))
    (`UserWidget.AddToViewport` (`self.PauseMenu`) 0)
    (`GameplayStatics.SetGamePaused` true)
    (`WidgetBlueprintLibrary.SetInputMode_UIOnlyEx` (`GameplayStatics.GetPlayerController` 0) (`self.PauseMenu`) "DoNotLock" true)))

(fn `UserConstructionScript`)