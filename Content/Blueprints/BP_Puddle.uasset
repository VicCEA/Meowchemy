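; BP_Puddle is an interactable puddle that reveals a hidden quest giver the first time it is used.
; Its construction script hides the linked QuestGiver mesh and disables the DialogueBox collision.
; Focus events toggle custom depth on the puddle mesh.
; Interact, gated by a DoOnce, unhides the quest giver, enables query-only collision on the dialogue box and spawns an enlarged poof effect at the quest giver's location.
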(event `/Game/Blueprints/Interaction/BPI_Interact.OnFocus`
  (`PrimitiveComponent.SetRenderCustomDepth` (`self.PuddleMesh`) true))

(event `/Game/Blueprints/Interaction/BPI_Interact.OnFocusEnd`
  (`PrimitiveComponent.SetRenderCustomDepth` (`self.PuddleMesh`) false))

(event `/Game/Blueprints/Interaction/BPI_Interact.Interact`
  (bind _questgiver (`self.QuestGiver`))
  (`/Engine/EditorBlueprintResources/StandardMacros.DoOnce` false
    (:`Completed`
      (`SceneComponent.SetHiddenInGame` (`Character.Mesh` _questgiver) false true)
      (`PrimitiveComponent.SetCollisionEnabled` (`/Game/Blueprints/Dialogue/BP_DialogueBox.Box` (`self.DialogueBox`)) "QueryOnly")
      (`NiagaraFunctionLibrary.SpawnSystemAtLocation` "/Game/Assets/Vfx/N_Poof.N_Poof" (`self.K2_GetActorLocation` _questgiver) (struct) (5.0 5.0 5.0)))))

(fn `UserConstructionScript`
  (`SceneComponent.SetHiddenInGame` (`Character.Mesh` (`self.QuestGiver`)) true true)
  (`PrimitiveComponent.SetCollisionEnabled` (`/Game/Blueprints/Dialogue/BP_DialogueBox.Box` (`self.DialogueBox`)) "NoCollision"))