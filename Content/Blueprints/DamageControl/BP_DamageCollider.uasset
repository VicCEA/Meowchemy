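; BP_DamageCollider is a sphere hit volume that damages and knocks back actors overlapping it, ignoring its owner.
; An overlap proceeds only if the target's CanBeDamaged flag is set, then clears that flag without restoring it here.
; Targets with BPC_FVS_Health lose the amount in the owner's BP_DamageComponent.
; Those that are PaperZD characters are also launched horizontally away from the owner.
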(event `self.ReceiveBeginPlay`
  (`PrimitiveComponent.IgnoreActorWhenMoving` (`self.Sphere`) (`self.GetOwner`) false))

(event `self.Sphere.OnComponentBeginOverlap`
  (params (OverlappedComponent :type "PrimitiveComponent Object Reference") (OtherActor :type "Actor Object Reference") (OtherComp :type "PrimitiveComponent Object Reference") (OtherBodyIndex :type Integer) (bFromSweep :type Boolean) (SweepResult :type "HitResult Structure (by ref)"))
  (if (not (== OtherActor (`self.GetOwner`)))
    (`self.ApplyDamage` OtherActor)))

(event `ApplyDamage`
  (params (OtherActor :type "Actor Object Reference"))
  (if (`Actor.bCanBeDamaged` OtherActor)
    (set `Actor.bCanBeDamaged` false OtherActor)
    (`self.DamageEffects` OtherActor)))

(event `DamageEffects`
  (params (LaunchTarget :type "Actor Object Reference"))
  (bind _returnvalue (`self.GetOwner`))
  (bind _returnvalue_2 (`self.GetComponentByClass` LaunchTarget "/Game/Blueprints/Abilities/Stats/BPC_FVS_Health.BPC_FVS_Health_C"))
  (bind (_returnvalue_x _returnvalue_y) (`KismetMathLibrary.BreakVector` (- (`self.K2_GetActorLocation` _returnvalue) (`self.K2_GetActorLocation` LaunchTarget))))
  (`/Engine/EditorBlueprintResources/StandardMacros.IsValid` _returnvalue_2
    (:`Is Valid`
      (`/Game/Blueprints/Abilities/Stats/BPC_FloatValueSystem.DecreaseValue` _returnvalue_2 (`/Game/Blueprints/DamageControl/BP_DamageComponent.Damage` (`self.GetComponentByClass` _returnvalue "/Game/Blueprints/DamageControl/BP_DamageComponent.BP_DamageComponent_C")))
      (bind _aspaper_zdcharacter (cast `PaperZDCharacter` LaunchTarget))
      (`Character.LaunchCharacter` _aspaper_zdcharacter (* (`KismetMathLibrary.Normal` (`KismetMathLibrary.MakeVector` _returnvalue_x _returnvalue_y)) -1500.0) true false))))

(fn `UserConstructionScript`)