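; Damage component for PaperZD characters that turns animation attack events into damage colliders or projectiles.
; On BeginPlay it identifies the owner's AnimBP (player, slime or ranged slime) and binds to its attack events.
; Melee attacks spawn a damage collider and destroy it on stop, with slimes also launched along the player-owner axis.
; Ranged slimes instead spawn a projectile oriented by their direction to the player.
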(event `StopAttack`
  (`Actor.K2_DestroyActor` (`self.Collider`)))

(event `self.ReceiveBeginPlay`
  (bind _aspaper_zdcharacter (cast `PaperZDCharacter` (`self.GetOwner`)))
  (bind _output_get (set `self.As Paper ZDCharacter` _aspaper_zdcharacter))
  (bind _returnvalue (`PaperZDCharacter.GetAnimInstance` _output_get))
  (bind _aszdanim_bp_character (cast `/Game/Paper2D/ZDAnimBP_Character` _returnvalue)
    (:`then`
      (set `self.Player` true)
      (add `/Game/Paper2D/ZDAnimBP_Character.EventStartAttack` _aszdanim_bp_character (delegate `StartAttack`))
      (add `/Game/Paper2D/ZDAnimBP_Character.EventStopAttack` _aszdanim_bp_character (delegate `StopAttack`)))
    (:`CastFailed`
      (set `self.Player` false)
      (bind _aszdanim_bp_simple_slime_enemy (cast `/Game/Paper2D/SlimeEnemy/ZDAnimBP_SimpleSlimeEnemy` _returnvalue)
        (:`then`
          (add `/Game/Paper2D/SlimeEnemy/ZDAnimBP_SimpleSlimeEnemy.OnStartAttack` _aszdanim_bp_simple_slime_enemy (delegate `StartAttack`))
          (add `/Game/Paper2D/SlimeEnemy/ZDAnimBP_SimpleSlimeEnemy.OnStopAttack` _aszdanim_bp_simple_slime_enemy (delegate `StopAttack`)))
        (:`CastFailed`
          (bind _aszdanim_bp_simple_slime_enemy_ranged (cast `/Game/Paper2D/SlimeEnemy/ZDAnimBP_SimpleSlimeEnemy_Ranged` _returnvalue))
          (add `/Game/Paper2D/SlimeEnemy/ZDAnimBP_SimpleSlimeEnemy_Ranged.OnStartAttack` _aszdanim_bp_simple_slime_enemy_ranged (delegate `ThrowProjectile`)))))))

(event `StartAttack`
  (bind _as_paper_zdcharacter (`self.As Paper ZDCharacter`))
  (if (not (`self.Player`))
    (`self.LaunchCharacterForward`))
  (bind _returnvalue (`|SpawnActorFromClass` "/Game/Blueprints/DamageControl/BP_DamageCollider.BP_DamageCollider_C" (`self.K2_GetComponentToWorld`) "Undefined" "OverrideRootScale" _as_paper_zdcharacter _as_paper_zdcharacter))
  (set `self.Collider` _returnvalue))

(event `LaunchCharacterForward`
  (`Character.LaunchCharacter` (`self.As Paper ZDCharacter`) (* (`/Game/Blueprints/FL_Utilities.CalculateDirectionBetweenTwoActors` (`GameplayStatics.GetPlayerCharacter` 0) (`self.GetOwner`)) 1000.0) false false))

(event `ThrowProjectile`
  (bind _returnvalue (`self.GetOwner`))
  (bind _as_paper_zdcharacter (`self.As Paper ZDCharacter`))
  (bind _returnvalue_2 (`|SpawnActorFromClass` "/Game/Blueprints/AI/Enemies/BP_EnemyProjectile.BP_EnemyProjectile_C" (`KismetMathLibrary.MakeTransform` (`Actor.K2_GetActorLocation` _returnvalue) (`KismetMathLibrary.Conv_VectorToRotator` (`/Game/Blueprints/FL_Utilities.CalculateDirectionBetweenTwoActors` _returnvalue (`GameplayStatics.GetPlayerPawn` 0)))) "AlwaysSpawn" "OverrideRootScale" _as_paper_zdcharacter _as_paper_zdcharacter))
  (set `self.Projectile` _returnvalue_2))