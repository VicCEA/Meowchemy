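; BP_DamageCollider is a sphere hitbox actor that damages and knocks back PaperZD characters and enemies it overlaps, ignoring its owner.
; Damageable targets become invulnerable, lose a fixed amount of BPC_FVS_Health and are launched horizontally away from the collider's owner.
; Characters also set IsHurt on their animation instance until a timer clears it and restores damageability.
; Enemies are never made damageable again here, and debug prints remain.
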(event `self.ReceiveBeginPlay`)

(event `self.Sphere.OnComponentBeginOverlap`
  (params (OverlappedComponent :type "PrimitiveComponent Object Reference") (OtherActor :type "Actor Object Reference") (OtherComp :type "PrimitiveComponent Object Reference") (OtherBodyIndex :type Integer) (bFromSweep :type Boolean) (SweepResult :type "HitResult Structure (by ref)"))
  (`KismetSystemLibrary.PrintString` (`KismetSystemLibrary.GetDisplayName` OtherActor) true true (struct :`R` 0.015756 :`G` 1.0 :`A` 1.0))
  (if (not (== OtherActor (`self.GetOwner`)))
    (`self.ApplyDamage` OtherActor)))

(event `ApplyDamage`
  (params (OtherActor :type "Actor Object Reference"))
  (if (`Actor.bCanBeDamaged` OtherActor)
    (bind _asbpzd_character (cast `/Game/Paper2D/BPZD_Character` OtherActor)
      (:`then`
        (set `Actor.bCanBeDamaged` false _asbpzd_character)
        (`self.DamageEffects` _asbpzd_character)
        (`self.CharacterDamage` _asbpzd_character))
      (:`CastFailed`
        (bind _asbpzd_enemy (cast `/Game/Blueprints/AI/Enemies/BPZD_Enemy` OtherActor))
        (`KismetSystemLibrary.PrintString` "DamagedEnemy" true true (struct :`G` 1.0 :`B` 0.151208 :`A` 1.0))
        (set `Actor.bCanBeDamaged` false _asbpzd_enemy)
        (`self.DamageEffects` _asbpzd_enemy)))))

(event `DamageEffects`
  (params (LaunchTarget :type "Character Object Reference"))
  (bind _returnvalue (`self.GetComponentByClass` LaunchTarget "/Game/Blueprints/Abilities/Stats/BPC_FVS_Health.BPC_FVS_Health_C"))
  (bind (_returnvalue_x _returnvalue_y) (`KismetMathLibrary.BreakVector` (- (`self.K2_GetActorLocation` (`self.GetOwner`)) (`self.K2_GetActorLocation` LaunchTarget))))
  (`/Engine/EditorBlueprintResources/StandardMacros.IsValid` _returnvalue
    (:`Is Valid`
      (`/Game/Blueprints/Abilities/Stats/BPC_FloatValueSystem.DecreaseValue` _returnvalue 10.0)
      (`Character.LaunchCharacter` LaunchTarget (* (`KismetMathLibrary.Normal` (`KismetMathLibrary.MakeVector` _returnvalue_x _returnvalue_y)) -2000.0) false false))))

(event `CharacterDamage`
  (params (Target :type "/Game/Paper2D/BPZD_Character Object Reference"))
  (bind _aszdanim_bp_character (cast `/Game/Paper2D/ZDAnimBP_Character` (`PaperZDAnimationComponent.AnimInstance` (`PaperZDCharacter.AnimationComponent` Target))))
  (set `/Game/Paper2D/ZDAnimBP_Character.IsHurt` true _aszdanim_bp_character)
  (`KismetSystemLibrary.K2_SetTimerDelegate` (delegate `EndHurt`) 1.0))

(event `EndHurt`
  (bind _aszdanim_bp_character (cast `/Game/Paper2D/ZDAnimBP_Character` (`PaperZDAnimationComponent.AnimInstance` (`PaperZDCharacter.AnimationComponent` (stale `CharacterDamage` Target)))))
  (set `/Game/Paper2D/ZDAnimBP_Character.IsHurt` false _aszdanim_bp_character)
  (set `Actor.bCanBeDamaged` true (stale `CharacterDamage` Target)))

(fn `UserConstructionScript`)