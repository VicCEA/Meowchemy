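; Swinging axe trap that sweeps back and forth and launches any BPZD_Character overlapping its box while running.
; The Moving timeline lerps rotation from StartPos at a rate set by Speed, with its Finished event alternating play and reverse.
; The launch is horizontal, scaled by LaunchForce from player 0's velocity rather than the axe's motion.
; Interacting pauses the trap for five seconds, and focus toggles a custom-depth highlight.
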(event `self.ReceiveBeginPlay`
  (`SceneComponent.K2_SetRelativeRotation` (`self.Scene`) (`self.StartPos`) false false)
  (`self.PlayAxe`))

(event `PlayAxe`
  (set `self.IsStopped` false)
  (bind (_direction _moving) (`Timeline|Moving` :!label _label)
    (:`Update`
      (`SceneComponent.K2_SetRelativeRotation` (`self.Scene`) (`KismetMathLibrary.RLerp` (`self.StartPos`) (struct :`Pitch` -90.0) _moving true) false false))
    (:`Finished`
      (if (`self.IsLooping`)
        (set `self.IsLooping` false)
        (`self.ReverseAxe`)
        (else
          (set `self.IsLooping` true)
          (`self.PlayAxe`))))))

(event `StopAxe`
  (set `self.IsStopped` true)
  (goto _label :!via `Stop`))

(event `ReverseAxe`
  (goto _label :!via `Reverse`))

(event `/Game/Blueprints/Interaction/BPI_Interact.Interact`
  (`self.StopAxe`)
  (`KismetSystemLibrary.K2_SetTimerDelegate` (delegate `PlayAxe`) 5.0))

(event `/Game/Blueprints/Interaction/BPI_Interact.OnFocus`
  (`PrimitiveComponent.SetRenderCustomDepth` (`self.StaticMesh`) true)
  (`PrimitiveComponent.SetRenderCustomDepth` (`self.Cube`) true))

(event `/Game/Blueprints/Interaction/BPI_Interact.OnFocusEnd`
  (`PrimitiveComponent.SetRenderCustomDepth` (`self.StaticMesh`) false)
  (`PrimitiveComponent.SetRenderCustomDepth` (`self.Cube`) false))

(event `self.Box.OnComponentBeginOverlap`
  (params (OverlappedComponent :type "PrimitiveComponent Object Reference") (OtherActor :type "Actor Object Reference") (OtherComp :type "PrimitiveComponent Object Reference") (OtherBodyIndex :type Integer) (bFromSweep :type Boolean) (SweepResult :type "HitResult Structure (by ref)"))
  (bind (_returnvalue_x _returnvalue_y) (`KismetMathLibrary.BreakVector` (* (`self.GetVelocity` (`GameplayStatics.GetPlayerCharacter` 0)) (`self.LaunchForce`))))
  (if (not (`self.IsStopped`))
    (bind _asbpzd_character (cast `/Game/Paper2D/BPZD_Character` OtherActor))
    (`Character.LaunchCharacter` _asbpzd_character (`KismetMathLibrary.MakeVector` _returnvalue_x _returnvalue_y) true false)))

(fn `UserConstructionScript`
  (`TimelineComponent.SetPlayRate` (`self.Moving`) (`self.Speed`)))