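; Lever switch trap Blueprint that toggles a linked ObjectToInteract when interacted with.
; Interact passes a DoOnce gate, checks the target for BPI_Interactables, then a FlipFlop alternates between sending start and stop messages.
; Gaining or losing focus toggles custom depth on the Cube and Box meshes and resets the gate, allowing one interaction until focus changes or ResetOnce fires.
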(event `/Game/Blueprints/Interaction/BPI_Interact.Interact`
  (bind _objecttointeract (`self.ObjectToInteract`))
  (`/Engine/EditorBlueprintResources/StandardMacros.DoOnce` false :!label _label
    (:`Completed`
      (if (`KismetSystemLibrary.DoesImplementInterface` _objecttointeract "/Game/Blueprints/Traps/BPI_Interactables.BPI_Interactables_C")
        (`/Engine/EditorBlueprintResources/StandardMacros.FlipFlop`
          (:`A`
            (message `/Game/Blueprints/Traps/BPI_Interactables.OnStart` _objecttointeract))
          (:`B`
            (message `/Game/Blueprints/Traps/BPI_Interactables.OnStop` _objecttointeract)))))))

(event `ResetOnce`
  (goto _label :!via `Reset`))

(event `/Game/Blueprints/Interaction/BPI_Interact.OnFocus`
  (`PrimitiveComponent.SetRenderCustomDepth` (`self.Cube`) true)
  (`PrimitiveComponent.SetRenderCustomDepth` (`self.Box`) true)
  (`self.ResetOnce`))

(event `/Game/Blueprints/Interaction/BPI_Interact.OnFocusEnd`
  (`PrimitiveComponent.SetRenderCustomDepth` (`self.Cube`) false)
  (`PrimitiveComponent.SetRenderCustomDepth` (`self.Box`) false)
  (`self.ResetOnce`))

(fn `UserConstructionScript`)