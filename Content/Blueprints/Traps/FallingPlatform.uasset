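; Falling platform trap that moves toward a reference end position after a BPZD_Character enters its trigger box, then returns after they leave.
; Each overlap event waits out a delay, then plays or reverses a timeline that lerps the platform between locations cached at BeginPlay, with speed set by FallDuration.
; The construction script applies shared mesh, scale and rotation to both platform and end reference, and moves the platform to the EndLocation variable.
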(event `self.ReceiveBeginPlay`
  (set `self.StartLocation` (`SceneComponent.RelativeLocation` (`self.MainPlatform`)))
  (set `self.EndLocation` (`SceneComponent.RelativeLocation` (`self.EndPlatformReference`))))

(event `self.Box.OnComponentBeginOverlap`
  (params (OverlappedComponent :type "PrimitiveComponent Object Reference") (OtherActor :type "Actor Object Reference") (OtherComp :type "PrimitiveComponent Object Reference") (OtherBodyIndex :type Integer) (bFromSweep :type Boolean) (SweepResult :type "HitResult Structure (by ref)"))
  (cast `/Game/Paper2D/BPZD_Character` OtherActor)
  (`KismetSystemLibrary.Delay` (`self.FallActivationDelay`))
  (`TimelineComponent.SetPlayRate` (`self.MovePlatform`) (/ 1.0 (`self.FallDuration`)))
  (bind (_direction _movetrack) (`Timeline|MovePlatform` :!label _label)
    (:`Update`
      (`SceneComponent.K2_SetRelativeLocation` (`self.MainPlatform`) (`KismetMathLibrary.VLerp` (`self.StartLocation`) (`self.EndLocation`) _movetrack) false false))))

(event `self.Box.OnComponentEndOverlap`
  (params (OverlappedComponent :type "PrimitiveComponent Object Reference") (OtherActor :type "Actor Object Reference") (OtherComp :type "PrimitiveComponent Object Reference") (OtherBodyIndex :type Integer))
  (cast `/Game/Paper2D/BPZD_Character` OtherActor)
  (`KismetSystemLibrary.Delay` 3.0)
  (`TimelineComponent.SetPlayRate` (`self.MovePlatform`) (/ 1.0 (`self.FallDuration`)))
  (goto _label :!via `Reverse`))

(fn `UserConstructionScript`
  (bind _mainplatform (`self.MainPlatform`))
  (bind _endplatformreference (`self.EndPlatformReference`))
  (bind _platformmesh (`self.PlatformMesh`))
  (`StaticMeshComponent.SetStaticMesh` _mainplatform _platformmesh)
  (`StaticMeshComponent.SetStaticMesh` _endplatformreference _platformmesh)
  (`SceneComponent.SetRelativeScale3D` _mainplatform (`self.PlatformSize`))
  (`SceneComponent.SetRelativeScale3D` _endplatformreference (`self.PlatformSize`))
  (`SceneComponent.K2_SetRelativeRotation` _endplatformreference (`self.PlatformRotation`) false false)
  (`SceneComponent.K2_SetRelativeRotation` _mainplatform (`self.PlatformRotation`) false false)
  (`SceneComponent.K2_SetRelativeLocation` _mainplatform (`self.EndLocation`) false false))