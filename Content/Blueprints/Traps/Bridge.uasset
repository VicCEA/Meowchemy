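; An interactable bridge trap that drops by swinging its two halves apart when Interact is called.
; A Timeline lerps the left and right scene components to opposite rotations, then reverses from the end after a delay.
; Because Finished also fires after reversing, that delayed reverse keeps repeating.
; Focus events toggle custom depth rendering on both halves for highlighting.
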(event `DropBridge`
  (bind (_direction _moving) (`Timeline|Timeline` :!label _label)
    (:`Update`
      (`SceneComponent.K2_SetRelativeRotation` (`self.SceneRight`) (`KismetMathLibrary.RLerp` (struct) (struct :`Pitch` -50.0) _moving) false false)
      (`SceneComponent.K2_SetRelativeRotation` (`self.SceneLeft`) (`KismetMathLibrary.RLerp` (struct) (struct :`Pitch` 50.0) _moving) false false))
    (:`Finished`
      (`KismetSystemLibrary.Delay` 5.0)
      (`self.ReverseBridge`))))

(event `ReverseBridge`
  (goto _label :!via `ReverseFromEnd`))

(event `/Game/Blueprints/Interaction/BPI_Interact.OnFocus`
  (`PrimitiveComponent.SetRenderCustomDepth` (`self.Left`) true)
  (`PrimitiveComponent.SetRenderCustomDepth` (`self.Right`) true))

(event `/Game/Blueprints/Interaction/BPI_Interact.OnFocusEnd`
  (`PrimitiveComponent.SetRenderCustomDepth` (`self.Left`) false)
  (`PrimitiveComponent.SetRenderCustomDepth` (`self.Right`) false))

(fn `Interact`
  (returns (DidInteract :type Boolean))
  (`self.DropBridge`)
  (return false))

(fn `UserConstructionScript`)