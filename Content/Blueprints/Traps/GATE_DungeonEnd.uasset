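; Dungeon-end gate Blueprint that moves its mesh when something overlaps the OnCharacterEnter trigger.
; BeginPlay caches the mesh's relative location as the origin.
; Each overlap plays the Moving timeline from the start, lerping the mesh from that origin to the NewLocation component's relative location.
; The overlap has no actor filter or one-shot guard, so re-entry restarts the motion from the origin.
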(event `self.ReceiveBeginPlay`
  (set `self.OriginLocation` (`SceneComponent.RelativeLocation` (`self.StaticMesh`))))

(event `self.OnCharacterEnter.OnComponentBeginOverlap`
  (params (OverlappedComponent :type "PrimitiveComponent Object Reference") (OtherActor :type "Actor Object Reference") (OtherComp :type "PrimitiveComponent Object Reference") (OtherBodyIndex :type Integer) (bFromSweep :type Boolean) (SweepResult :type "HitResult Structure (by ref)"))
  (bind (_direction _moving) (`Timeline|Moving` :!via `PlayFromStart`)
    (:`Update`
      (`SceneComponent.K2_SetRelativeLocation` (`self.StaticMesh`) (`KismetMathLibrary.VLerp` (`self.OriginLocation`) (`SceneComponent.RelativeLocation` (`self.NewLocation`)) _moving) false false))))

(fn `NewFunction`)

(fn `UserConstructionScript`)