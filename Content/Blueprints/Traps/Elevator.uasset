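; Elevator in the Traps folder that slides its static mesh between its starting position and a target point.
; BeginPlay caches the mesh's relative location, and the Moving timeline lerps from it to the NewLocation component's relative location without sweeping.
; OnStart plays the timeline from the start, while OnStop reverses it from the end, so neither resumes from the current position.
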(event `self.ReceiveBeginPlay`
  (set `self.OriginLocation` (`SceneComponent.RelativeLocation` (`self.StaticMesh`))))

(event `/Game/Blueprints/Traps/BPI_Interactables.OnStart`
  (bind (_direction _moving) (`Timeline|Moving` :!via `PlayFromStart` :!label _label)
    (:`Update`
      (`SceneComponent.K2_SetRelativeLocation` (`self.StaticMesh`) (`KismetMathLibrary.VLerp` (`self.OriginLocation`) (`SceneComponent.RelativeLocation` (`self.NewLocation`)) _moving) false false))))

(event `/Game/Blueprints/Traps/BPI_Interactables.OnStop`
  (goto _label :!via `ReverseFromEnd`))

(fn `NewFunction`)

(fn `UserConstructionScript`)