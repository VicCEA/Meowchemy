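; BP_GoldenPath is an actor that draws a live navigation path from its own location to the player character using spline meshes.
; Every Tick it runs a synchronous pathfinding query and passes the result to UpdatePath, with no throttling.
; UpdatePath destroys the previous segments, loads the path points into the spline in local space, and adds spline mesh components shaped by neighboring points' locations and tangents.
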(event `self.ReceiveBeginPlay`)

(event `self.ReceiveTick`
  (params (DeltaSeconds :type "Float (single-precision)"))
  (bind _returnvalue (`NavigationSystemV1.FindPathToActorSynchronously` (`self.K2_GetActorLocation`) (`GameplayStatics.GetPlayerCharacter` 0) 50.0 null null))
  (bind _output_get (set `self.Path` _returnvalue))
  (`self.UpdatePath` _output_get "NewPath"))

(event `UpdatePath`
  (params (AffectedPath :type "NavigationPath Object Reference") (PathEvent :type "ENavPathEvent Enum" :default "Cleared"))
  (bind _spline (`self.Spline`))
  (bind _pathpoints (`NavigationPath.PathPoints` AffectedPath))
  (`self.ClearPoints`)
  (`SplineComponent.SetSplinePoints` (`self.Spline`) _pathpoints "Local" true)
  (for (_ _array_index) _pathpoints
    (bind _returnvalue (`AddComponent|NODE_AddSplineMeshComponent-1`))
    (`KismetArrayLibrary.Array_Add` (`self.Points`) _returnvalue)
    (bind (_location _tangent) (`SplineComponent.GetLocationAndTangentAtSplinePoint` _spline (- _array_index 1) "Local"))
    (bind (_location_2 _tangent_2) (`SplineComponent.GetLocationAndTangentAtSplinePoint` _spline _array_index "Local"))
    (`SplineMeshComponent.SetStartAndEnd` _returnvalue _location _tangent _location_2 _tangent_2 true)))

(event `ClearPoints`
  (if (> (`KismetArrayLibrary.Array_Length` (`self.Points`)) 0)
    (for _array_element (`self.Points`)
      (`ActorComponent.K2_DestroyComponent` _array_element))
    (`KismetArrayLibrary.Array_Clear` (`self.Points`))))

(fn `UserConstructionScript`)