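; Trigger actor that starts location-specific background music when a player character enters it and stops it when that character leaves.
; Begin and end overlap events run only with authority and act only on a BPZD_Character controlled by a MyPlayerController.
; That controller receives the start or stop call with the trigger's BackgroundMusic variable, so the controller handles the music per player.
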(event `self.ReceiveActorBeginOverlap`
  (params (OtherActor :type "Actor Object Reference"))
  (`/Engine/EditorBlueprintResources/ActorMacros.Switch Has Authority`
    (:`Authority`
      (bind _asbpzd_character (cast `/Game/Paper2D/BPZD_Character` OtherActor))
      (bind _asmy_player_controller (cast `/Game/Blueprints/MyPlayerController` (`Pawn.GetController` _asbpzd_character)))
      (`/Game/Blueprints/MyPlayerController.StartLocalizedBackgroundMusic` _asmy_player_controller (`self.BackgroundMusic`)))))

(event `self.ReceiveActorEndOverlap`
  (params (OtherActor :type "Actor Object Reference"))
  (`/Engine/EditorBlueprintResources/ActorMacros.Switch Has Authority`
    (:`Authority`
      (bind _asbpzd_character (cast `/Game/Paper2D/BPZD_Character` OtherActor))
      (bind _asmy_player_controller (cast `/Game/Blueprints/MyPlayerController` (`Pawn.GetController` _asbpzd_character)))
      (`/Game/Blueprints/MyPlayerController.StopLocalizedBackgroundMusic` _asmy_player_controller (`self.BackgroundMusic`)))))

(fn `UserConstructionScript`)