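; BP_KillVolume is a hazard volume, water or lava, that punishes characters and enemies overlapping its box.
; Player characters lose a little health and teleport to the respawn transform stored on the Meowchemy game mode.
; Enemies instead take a heavy health hit through the same health component.
; Both trigger an attenuated sound at their location, a sizzle or a splash depending on the Lava flag.
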(event `self.Box.OnComponentBeginOverlap`
  (params (OverlappedComponent :type "PrimitiveComponent Object Reference") (OtherActor :type "Actor Object Reference") (OtherComp :type "PrimitiveComponent Object Reference") (OtherBodyIndex :type Integer) (bFromSweep :type Boolean) (SweepResult :type "HitResult Structure (by ref)"))
  (bind _asbpzd_character (cast `/Game/Paper2D/BPZD_Character` OtherActor)
    (:`then`
      (`self.PlaySound` (`self.K2_GetActorLocation` _asbpzd_character))
      (`/Game/Blueprints/Abilities/Stats/BPC_FloatValueSystem.DecreaseValue` (`/Game/Paper2D/BPZD_Character.BPC_FVS_Health` _asbpzd_character) 5.0)
      (bind _asbpgm_meowchemy_game_mode (cast `/Game/Blueprints/BPGM_MeowchemyGameMode` (`GameplayStatics.GetGameMode`)))
      (bind (_respawn_transform_location _respawn_transform_rotation) (`KismetMathLibrary.BreakTransform` (`/Game/Blueprints/BPGM_MeowchemyGameMode.Respawn Transform` _asbpgm_meowchemy_game_mode)))
      (`self.K2_TeleportTo` _asbpzd_character _respawn_transform_location _respawn_transform_rotation))
    (:`CastFailed`
      (bind _asbpzd_enemy (cast `/Game/Blueprints/AI/Enemies/BPZD_Enemy` OtherActor))
      (`/Game/Blueprints/Abilities/Stats/BPC_FloatValueSystem.DecreaseValue` (`/Game/Blueprints/AI/Enemies/BPZD_Enemy.BPC_FVS_Health` _asbpzd_enemy) 100.0)
      (`self.PlaySound` (`self.K2_GetActorLocation` _asbpzd_enemy)))))

(event `PlaySound`
  (params (Location :type "Vector Structure"))
  (if (`self.Lava`)
    (`GameplayStatics.PlaySoundAtLocation` "/Game/Sounds/133449__chaosportal__cigarette-sizzle-02.133449__chaosportal__cigarette-sizzle-02" Location (struct) 5.0 1.0 0.0 "/Game/Sounds/SA_SFX.SA_SFX" null null null)
    (else
      (`GameplayStatics.PlaySoundAtLocation` "/Game/Sounds/628459__timkahn__watrsplsh_rock-splash-14_tk_sassmkh8020.628459__timkahn__watrsplsh_rock-splash-14_tk_sassmkh8020" Location (struct) 3.0 1.0 0.0 "/Game/Sounds/SA_SFX.SA_SFX" null null null))))

(fn `UserConstructionScript`)