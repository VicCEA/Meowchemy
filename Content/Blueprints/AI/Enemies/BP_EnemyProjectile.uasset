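; Enemy projectile actor that damages the player character type (BPZD_Character) when its sphere overlaps one.
; On BeginPlay the sphere ignores its owner and itself when moving, and a timer destroys the projectile after a fixed lifetime.
; An overlap with that character decreases its health component's value and destroys the projectile.
; Other overlaps effectively leave it alive, as that branch destroys it only when self is invalid.
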(event `self.ReceiveBeginPlay`
  (bind _sphere (`self.Sphere`))
  (`PrimitiveComponent.IgnoreActorWhenMoving` _sphere (`self.GetOwner`) true)
  (`PrimitiveComponent.IgnoreActorWhenMoving` (`self.Sphere`) self true)
  (`PrimitiveComponent.IgnoreComponentWhenMoving` _sphere (`self.Sphere`) true)
  (bind _returnvalue (`KismetSystemLibrary.K2_SetTimerDelegate` (delegate `destroyProjectile`) 5.0))
  (set `self.Timer` _returnvalue))

(event `destroyProjectile`
  (`KismetSystemLibrary.K2_ClearAndInvalidateTimerHandle` (`self.Timer`))
  (`self.K2_DestroyActor`))

(event `self.Sphere.OnComponentBeginOverlap`
  (params (OverlappedComponent :type "PrimitiveComponent Object Reference") (OtherActor :type "Actor Object Reference") (OtherComp :type "PrimitiveComponent Object Reference") (OtherBodyIndex :type Integer) (bFromSweep :type Boolean) (SweepResult :type "HitResult Structure (by ref)"))
  (bind _asbpzd_character (cast `/Game/Paper2D/BPZD_Character` OtherActor)
    (:`then`
      (`/Game/Blueprints/Abilities/Stats/BPC_FloatValueSystem.DecreaseValue` (`/Game/Paper2D/BPZD_Character.BPC_FVS_Health` _asbpzd_character) 10.0)
      (`self.destroyProjectile`))
    (:`CastFailed`
      (`/Engine/EditorBlueprintResources/StandardMacros.IsValid` self
        (:`Is Not Valid`
          (`self.destroyProjectile`))))))

(fn `UserConstructionScript`)