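; Actor component that keeps an AI-controlled owner facing one of two opposite directions along its spawn forward axis.
; BeginPlay caches the owner's rotation, and Tick sets the AI controller's focal point ahead of or behind the owner along that axis.
; The sign of world Y velocity picks the side: positive looks opposite the spawn forward, negative along it, and zero leaves the focus unchanged.
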(event `self.ReceiveBeginPlay`
  (set `self.SpawnRotation` (`Actor.K2_GetActorRotation` (`self.GetOwner`))))

(event `self.ReceiveTick`
  (params (DeltaSeconds :type "Float (single-precision)"))
  (bind _returnvalue (`self.GetOwner`))
  (bind _returnvalue_2 (`AIBlueprintHelperLibrary.GetAIController` _returnvalue))
  (bind _returnvalue_3 (`Actor.K2_GetActorLocation` _returnvalue))
  (bind (_returnvalue_x _returnvalue_y) (`KismetMathLibrary.BreakVector` (`Actor.GetVelocity` _returnvalue)))
  (bind _returnvalue_4 (* (`KismetMathLibrary.GetForwardVector` (`self.SpawnRotation`)) 100.0))
  (`/Engine/EditorBlueprintResources/StandardMacros.IsValid` _returnvalue_2
    (:`Is Valid`
      (`/Engine/EditorBlueprintResources/StandardMacros.CompareFloat` _returnvalue_y
        (:`>`
          (`AIController.K2_SetFocalPoint` _returnvalue_2 (+ _returnvalue_3 (* _returnvalue_4 -1.0))))
        (:`<`
          (`AIController.K2_SetFocalPoint` _returnvalue_2 (+ _returnvalue_3 _returnvalue_4)))))))