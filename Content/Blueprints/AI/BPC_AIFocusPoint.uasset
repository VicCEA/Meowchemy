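; Actor component that keeps an AI-controlled PaperZD character's focal point ahead of or behind it according to its movement direction.
; At BeginPlay it caches the owner's spawn rotation and character reference.
; Each tick, the sign of normalized Y velocity places the AI controller's focal point a fixed distance along or against the spawn forward vector.
; Zero Y velocity leaves the last focal point in place.
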(event `self.ReceiveBeginPlay`
  (set `self.SpawnRotation` (`Actor.K2_GetActorRotation` (`self.GetOwner`)))
  (bind _aspaper_zdcharacter (cast `PaperZDCharacter` (`self.GetOwner`)))
  (set `self.As Paper ZDCharacter` _aspaper_zdcharacter))

(event `self.ReceiveTick`
  (params (DeltaSeconds :type "Float (single-precision)"))
  (bind (_returnvalue_x _returnvalue_y) (`KismetMathLibrary.BreakVector` (`KismetMathLibrary.Normal` (`Actor.GetVelocity` (`self.As Paper ZDCharacter`)))))
  (`self.UpdateControlRotation` _returnvalue_y))

(event `UpdateControlRotation`
  (params (Input :type "Float (double-precision)"))
  (`/Engine/EditorBlueprintResources/StandardMacros.CompareFloat` Input
    (:`>`
      (`self.SetCharacterFocalPoint` 100.0))
    (:`<`
      (`self.SetCharacterFocalPoint` -100.0))))

(event `SetCharacterFocalPoint`
  (params (FocalPointDistance :type "Float (single-precision)"))
  (bind _returnvalue (`self.GetOwner`))
  (bind _returnvalue_2 (`AIBlueprintHelperLibrary.GetAIController` (`Pawn.GetController` (`Actor.Instigator` _returnvalue))))
  (`/Engine/EditorBlueprintResources/StandardMacros.IsValid` _returnvalue_2
    (:`Is Valid`
      (`AIController.K2_SetFocalPoint` _returnvalue_2 (+ (`Actor.K2_GetActorLocation` _returnvalue) (* (`KismetMathLibrary.GetForwardVector` (`self.SpawnRotation`)) FocalPointDistance))))))