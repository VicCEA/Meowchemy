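; Game mode for Meowchemy that handles respawning the player.
; RespawnPlayer spawns a fresh actor of the passed object's class at the stored respawn transform, has player controller 0 possess it, then enables input and damage.
; It then rebinds the HUD widget's events and calls OnRespawn on the new BPZD_Character, stopping early if either cast fails.
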(fn `RespawnPlayer`
  (params (Object :type "Character Object Reference"))
  (locals (NewPlayer :type "Character Object Reference"))
  (bind _returnvalue (`GameplayStatics.GetPlayerController` 0))
  (bind _returnvalue_2 (`|SpawnActorFromClass` (`GameplayStatics.GetObjectClass` Object) (`self.Respawn Transform`) "Undefined" "OverrideRootScale" null null))
  (bind _output_get (set `local.NewPlayer` _returnvalue_2))
  (`Controller.Possess` (`GameplayStatics.GetPlayerController` 0) _output_get)
  (`self.EnableInput` _returnvalue)
  (set `self.bCanBeDamaged` true)
  (bind _ashud_player_hud (cast `/Game/UI/HUD_PlayerHud` (`PlayerController.GetHUD` _returnvalue)))
  (`/Game/UI/WI_PlayerHUD.BindEvents` (`/Game/UI/HUD_PlayerHud.HudWidget` _ashud_player_hud))
  (bind _asbpzd_character (cast `/Game/Paper2D/BPZD_Character` (`local.NewPlayer`)))
  (`/Game/Paper2D/BPZD_Character.OnRespawn` _asbpzd_character))

(fn `UserConstructionScript`)