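; BP_Vortex is a short-lived vortex ability actor that damages zombie-type enemies and exerts radial force on its surroundings.
; A timer set on BeginPlay destroys it after a few seconds, while Tick fires a RadialForce impulse every frame.
; Its Sphere overlap casts to BPZD_Enemy and subtracts a fixed amount from that enemy's health component.
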(event `self.ReceiveBeginPlay`
  (`KismetSystemLibrary.K2_SetTimerDelegate` (delegate `Destroy`) 3.0))

(event `self.ReceiveActorBeginOverlap`
  (params (OtherActor :type "Actor Object Reference")))

(event `Destroy`
  (`self.K2_DestroyActor`))

(event `self.ReceiveTick`
  (params (DeltaSeconds :type "Float (single-precision)"))
  (`RadialForceComponent.FireImpulse` (`self.RadialForce`)))

(event `self.Sphere.OnComponentBeginOverlap`
  (params (OverlappedComponent :type "PrimitiveComponent Object Reference") (OtherActor :type "Actor Object Reference") (OtherComp :type "PrimitiveComponent Object Reference") (OtherBodyIndex :type Integer) (bFromSweep :type Boolean) (SweepResult :type "HitResult Structure (by ref)"))
  (bind _asbpzd_enemy (cast `/Game/Blueprints/AI/Enemies/BPZD_Enemy` OtherActor))
  (`/Game/Blueprints/Abilities/Stats/BPC_FloatValueSystem.DecreaseValue` (`/Game/Blueprints/AI/Enemies/BPZD_Enemy.BPC_FVS_Health` _asbpzd_enemy) 80.0))

(fn `UserConstructionScript`)