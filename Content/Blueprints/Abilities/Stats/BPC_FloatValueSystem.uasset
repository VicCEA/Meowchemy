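; BPC_FloatValueSystem is a reusable stat component that tracks a float current value between zero and a maximum.
; Increase and decrease functions clamp the value to that range and fire the matching increased or decreased event dispatcher.
; A decrease that reaches zero also fires a depleted event.
; Resetting to max reuses the increase function, so it broadcasts as an increase.
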(fn `DecreaseValue`
  (params (Value :type "Float (double-precision)"))
  (bind _returnvalue (- (`self.CurrentValue`) Value))
  (if (<= _returnvalue 0.0)
    (set `self.CurrentValue` 0.0)
    (`self.OnValueDecreased`)
    (`self.OnValueDepleted`)
    (else
      (set `self.CurrentValue` _returnvalue)
      (`self.OnValueDecreased`))))

(fn `IncreaseVlaue`
  (params (Value :type "Float (double-precision)"))
  (bind _maxvalue (`self.MaxValue`))
  (bind _returnvalue (+ (`self.CurrentValue`) Value))
  (if (>= _returnvalue _maxvalue)
    (set `self.CurrentValue` _maxvalue)
    (`self.OnValueIncreased`)
    (else
      (set `self.CurrentValue` _returnvalue)
      (`self.OnValueIncreased`))))

(fn `ResetToMaxValue`
  (`self.IncreaseVlaue` (`self.MaxValue`)))