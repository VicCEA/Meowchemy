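; Component on BPZD_Character that turns attack and dash input into abilities, each added to the owner as an ability component.
; With none active, input starts Attack1 or a grounded dash immediately.
; Attack presses during Attack1 or Attack2 store the next combo step in BufferedAbility.
; AbilityBuffer calls while busy copy that stored step, not the requested ability, into an empty NextAbility, which OnAbilityEnd starts.
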(event `EnhancedInput|/Game/Input/IA_Attack`
  (params (ActionValue :type Boolean) (ElapsedSeconds :type "Float (double-precision)") (TriggeredSeconds :type "Float (double-precision)") (InputAction :type "InputAction Object Reference" :default "/Game/Input/IA_Attack.IA_Attack"))
  (:`Started`
    (if (`self.CheckForAbility`)
      (if (== (`self.CurrentAbility`) "/Game/Blueprints/Abilities/BPC_Ability_Attack1.BPC_Ability_Attack1_C")
        (set `self.BufferedAbility` "/Game/Blueprints/Abilities/BPC_Ability_Attack2.BPC_Ability_Attack2_C")
        (elif (== (`self.CurrentAbility`) "/Game/Blueprints/Abilities/BPC_Ability_Attack2.BPC_Ability_Attack2_C")
          (set `self.BufferedAbility` "/Game/Blueprints/Abilities/BPC_Ability_Attack3.BPC_Ability_Attack3_C")))
      (else
        (`self.AbilityBuffer` "/Game/Blueprints/Abilities/BPC_Ability_Attack1.BPC_Ability_Attack1_C")))))

(event `EnhancedInput|/Game/Input/IA_Dash`
  (params (ActionValue :type Boolean) (ElapsedSeconds :type "Float (double-precision)") (TriggeredSeconds :type "Float (double-precision)") (InputAction :type "InputAction Object Reference" :default "/Game/Input/IA_Dash.IA_Dash"))
  (:`Started`
    (bind _asbpzd_character (cast `/Game/Paper2D/BPZD_Character` (`self.GetOwner`)))
    (if (not (`NavMovementComponent.IsFalling` (`Character.CharacterMovement` _asbpzd_character)))
      (`self.AbilityBuffer` "/Game/Blueprints/Abilities/BPC_Ability_Dash.BPC_Ability_Dash_C"))))

(event `AbilityBuffer`
  (params (NewAbility :type "ActorComponent Class Reference"))
  (if (`self.CheckForAbility`)
    (if (not (`KismetSystemLibrary.IsValidClass` (`self.NextAbility`)))
      (set `self.NextAbility` (`self.BufferedAbility`)))
    (else
      (set `self.NextAbility` NewAbility)
      (`self.SetAbility`))))

(fn `CheckForAbility`
  (returns (HasAbility :type Boolean))
  (bind _asbpzd_character (cast `/Game/Paper2D/BPZD_Character` (`self.GetOwner`)))
  (return (`KismetSystemLibrary.IsValid` (`Actor.GetComponentByClass` _asbpzd_character "/Game/Blueprints/Abilities/BPC_Ability_Base.BPC_Ability_Base_C"))))

(fn `OnAbilityEnd`
  (if (`KismetSystemLibrary.IsValidClass` (`self.NextAbility`))
    (`self.SetAbility`)))

(fn `SetAbility`
  (bind _nextability (`self.NextAbility`))
  (`|AddComponentByClass` (`self.GetOwner`) _nextability)
  (set `self.CurrentAbility` _nextability)
  (set `self.NextAbility` null))