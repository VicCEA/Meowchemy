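; Actor component that makes its owning actor, presumably a companion, follow the player character.
; On BeginPlay it caches the first player's BPZD_Character.
; Each tick it lerps the owner's location toward that character's CompanionLocation component using DeltaSeconds times Speed, giving an eased follow.
; Movement sets location directly without sweep, so it ignores collision along the path and leaves rotation untouched.
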(event `self.ReceiveBeginPlay`
  (`parent.ReceiveBeginPlay`)
  (bind _asbpzd_character (cast `/Game/Paper2D/BPZD_Character` (`GameplayStatics.GetPlayerCharacter` 0)))
  (set `self.As BPZD Character` _asbpzd_character))

(event `self.ReceiveTick`
  (params (DeltaSeconds :type "Float (single-precision)"))
  (bind _returnvalue (`self.GetOwner`))
  (`parent.ReceiveTick` DeltaSeconds)
  (`Actor.K2_SetActorLocation` _returnvalue (`KismetMathLibrary.VLerp` (`Actor.K2_GetActorLocation` _returnvalue) (`SceneComponent.K2_GetComponentLocation` (`/Game/Paper2D/BPZD_Character.CompanionLocation` (`self.As BPZD Character`))) (* DeltaSeconds (`self.Speed`))) false false))