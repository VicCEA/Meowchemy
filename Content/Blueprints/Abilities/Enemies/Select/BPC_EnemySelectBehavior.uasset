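; Enemy actor component that picks the next ability, attack or follow, for its BPZD_Enemy owner.
; On BeginPlay it caches the enemy's player distance and ability control, then binds selection to the attack cooldown's end, or selects once immediately if no cooldown component exists.
; Selection queues the attack component when the player is within range and CanAttack is set, otherwise the follow component.
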(event `self.ReceiveBeginPlay`
  (bind _returnvalue (`self.GetOwner`))
  (bind _returnvalue_2 (`Actor.GetComponentByClass` _returnvalue "/Game/Blueprints/Abilities/BP_AbilityControl.BP_AbilityControl_C"))
  (bind _returnvalue_3 (`Actor.GetComponentByClass` (`self.GetOwner`) "/Game/Blueprints/Abilities/Enemies/BPC_EnemyAttackCooldown.BPC_EnemyAttackCooldown_C"))
  (`parent.ReceiveBeginPlay`)
  (bind _asbpzd_enemy (cast `/Game/Blueprints/AI/Enemies/BPZD_Enemy` _returnvalue))
  (set `self.PlayerDistance` (`/Game/Blueprints/AI/Enemies/BPZD_Enemy.PlayerDistance` _asbpzd_enemy))
  (`/Engine/EditorBlueprintResources/StandardMacros.IsValid` _returnvalue_2
    (:`Is Valid`
      (set `self.AbilityControl` _returnvalue_2)
      (`/Engine/EditorBlueprintResources/StandardMacros.IsValid` _returnvalue_3
        (:`Is Valid`
          (add `/Game/Blueprints/Abilities/Enemies/BPC_EnemyAttackCooldown.OnEndCooldown` _returnvalue_3 (delegate `OnCooldownEnd`)))
        (:`Is Not Valid`
          (`self.SelectBehaviour`))))))

(event `self.ReceiveTick`
  (params (DeltaSeconds :type "Float (single-precision)"))
  (`parent.ReceiveTick` DeltaSeconds))

(event `OnCooldownEnd`
  (`self.SelectBehaviour`))

(event `SelectBehaviour`
  (bind _abilitycontrol (`self.AbilityControl`))
  (if (<= (`Actor.GetDistanceTo` (`self.GetOwner`) (`GameplayStatics.GetPlayerPawn` 0)) (`self.PlayerDistance`))
    (if (`self.CanAttack`)
      (`/Game/Blueprints/Abilities/BP_AbilityControl.SetNextAbility` _abilitycontrol (`self.AttackComponent`))
      (else
        (`/Game/Blueprints/Abilities/BP_AbilityControl.SetNextAbility` _abilitycontrol (`self.FollowComponent`) :!label _label)))
    (else
      (goto _label))))