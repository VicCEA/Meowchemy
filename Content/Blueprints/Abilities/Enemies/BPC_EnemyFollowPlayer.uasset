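; Enemy ability component that sends its owning AI toward the first player's pawn.
; On BeginPlay it issues a single AI MoveTo on the owner's controller, with continuous goal tracking and an acceptance radius, printing a debug message if the request fails.
; Tick only calls the parent; the range check and the logic to buffer the next ability and remove the component are unconnected.
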(event `self.ReceiveBeginPlay`
  (`parent.ReceiveBeginPlay`)
  (`self.GoToPlayer`))

(event `self.ReceiveTick`
  (params (DeltaSeconds :type "Float (single-precision)"))
  (`parent.ReceiveTick` DeltaSeconds))

(event `GoToPlayer`
  (`AITask_MoveTo.AIMoveTo` (`AIBlueprintHelperLibrary.GetAIController` (`self.GetOwner`)) (0.0 0.0 0.0) (`GameplayStatics.GetPlayerPawn` 0) (`self.Acceptance Radius`) "Default" "Default" true true true
    (:`OnRequestFailed`
      (`KismetSystemLibrary.PrintString` "Failed"))))