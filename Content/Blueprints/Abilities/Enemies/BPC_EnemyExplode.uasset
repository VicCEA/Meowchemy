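; Enemy ability component that, despite its Explode name, applies a one-shot damage and launch to its owner on BeginPlay.
; If the owner can be damaged, it clears that flag, never restoring it here, and deducts a fixed amount through BPC_FVS_Health.
; With that health component present, a PaperZD character owner is then launched horizontally toward the player, using a negated player-to-owner direction.
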(event `self.ReceiveBeginPlay`
  (bind _returnvalue (`self.GetOwner`))
  (bind _returnvalue_2 (`self.GetOwner`))
  (bind _returnvalue_3 (`Actor.GetComponentByClass` _returnvalue_2 "/Game/Blueprints/Abilities/Stats/BPC_FVS_Health.BPC_FVS_Health_C"))
  (bind (_returnvalue_x _returnvalue_y) (`KismetMathLibrary.BreakVector` (- (`Actor.K2_GetActorLocation` _returnvalue_2) (`Actor.K2_GetActorLocation` (`GameplayStatics.GetPlayerCharacter` 0)))))
  (`parent.ReceiveBeginPlay`)
  (if (`Actor.bCanBeDamaged` _returnvalue)
    (set `Actor.bCanBeDamaged` false _returnvalue)
    (`/Engine/EditorBlueprintResources/StandardMacros.IsValid` _returnvalue_3
      (:`Is Valid`
        (`/Game/Blueprints/Abilities/Stats/BPC_FloatValueSystem.DecreaseValue` _returnvalue_3 50.0)
        (bind _aspaper_zdcharacter (cast `PaperZDCharacter` _returnvalue_2))
        (`Character.LaunchCharacter` _aspaper_zdcharacter (* (`KismetMathLibrary.Normal` (`KismetMathLibrary.MakeVector` _returnvalue_x _returnvalue_y)) -1500.0) true false)))))