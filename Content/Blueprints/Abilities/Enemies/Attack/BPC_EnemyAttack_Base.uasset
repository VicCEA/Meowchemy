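; Base enemy attack ability component for BPZD_Enemy that runs one attack toward the player, timed by flipbook duration.
; On BeginPlay it resets sprite color, sets IsAttack on the SimpleSlimeEnemy anim instance, and turns the AI controller and disc toward the player on XY.
; The disc is optionally shown during the attack.
; When the timer ends, it clears the attack, adds a cooldown and hands the next ability to BPAbilityControl.
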(event `self.ReceiveBeginPlay`
  (`parent.ReceiveBeginPlay`)
  (bind _asbpzd_enemy (cast `/Game/Blueprints/AI/Enemies/BPZD_Enemy` (`self.GetOwner`)))
  (set `self.As BPZD Enemy` _asbpzd_enemy)
  (`self.PlayAnimation`)
  (`KismetSystemLibrary.K2_SetTimerDelegate` (delegate `self.RemoveComponent`) (`/Game/Blueprints/FL_Utilities.CalculateFlipbookDuration` (`self.AnimationFrames`))))

(event `self.RemoveComponent`
  (`self.StopAnimation`)
  (`self.EndAbility`))

(event `self.PlayAnimation`
  (`PaperFlipbookComponent.SetSpriteColor` (`PaperCharacter.Sprite` (`self.As BPZD Enemy`)) (struct :`R` 1.0 :`G` 1.0 :`B` 1.0 :`A` 1.0))
  (`self.SetAttack` true)
  (`self.ApplyEffect`))

(event `self.ApplyEffect`
  (bind _as_bpzd_enemy (`self.As BPZD Enemy`))
  (bind _returnvalue (`KismetMathLibrary.Conv_VectorToRotator` (`KismetMathLibrary.MakeVector` (.x (`/Game/Blueprints/FL_Utilities.CalculateDirectionBetweenTwoActors` (`self.GetOwner`) (`GameplayStatics.GetPlayerCharacter` 0))) (.y (`/Game/Blueprints/FL_Utilities.CalculateDirectionBetweenTwoActors` (`self.GetOwner`) (`GameplayStatics.GetPlayerCharacter` 0))))))
  (`self.HideDisc` false)
  (`Controller.SetControlRotation` (`AIBlueprintHelperLibrary.GetAIController` _as_bpzd_enemy) _returnvalue)
  (`/Game/Blueprints/AI/Enemies/BPZD_Enemy.RotateDisc` _as_bpzd_enemy (`KismetMathLibrary.Conv_RotatorToVector` _returnvalue)))

(event `self.StopAnimation`
  (`self.SetAttack` false)
  (`self.HideDisc` true))

(event `HideDisc`
  (params (NewHidden :type Boolean))
  (if (`self.ShowDisc`)
    (`SceneComponent.SetHiddenInGame` (`/Game/Blueprints/AI/Enemies/BPZD_Enemy.Disc` (`self.As BPZD Enemy`)) NewHidden false)))

(event `self.EndAbility`
  (bind _as_bpzd_enemy (`self.As BPZD Enemy`))
  (`|AddComponentByClass` _as_bpzd_enemy "/Game/Blueprints/Abilities/Enemies/BPC_EnemyAttackCooldown.BPC_EnemyAttackCooldown_C")
  (`/Game/Blueprints/Abilities/BP_AbilityControl.SetNextAbility` (`/Game/Blueprints/AI/Enemies/BPZD_Enemy.BP_AbilityControl` _as_bpzd_enemy) (`self.SelectComponent`)))

(event `SetAttack`
  (params (IsAttack :type Boolean))
  (bind _aszdanim_bp_simple_slime_enemy (cast `/Game/Paper2D/SlimeEnemy/ZDAnimBP_SimpleSlimeEnemy` (`PaperZDCharacter.GetAnimInstance` (`self.As BPZD Enemy`))))
  (set `/Game/Paper2D/SlimeEnemy/ZDAnimBP_SimpleSlimeEnemy.IsAttack` IsAttack _aszdanim_bp_simple_slime_enemy))

(event `self.ReceiveTick`
  (params (DeltaSeconds :type "Float (single-precision)")))