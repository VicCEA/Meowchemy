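; Enemy actor component that picks the owner's next ability, either following or attacking the player.
; On BeginPlay it caches the owner's BP_AbilityControl and runs SelectBehaviour, which passes the choice to SetNextAbility.
; Attack is chosen only when the player is within close range and no BPC_EnemyAttackCooldown component is present, so that component's presence acts as the cooldown flag.
; A BPC_EnemyDamage check exists but is disconnected.
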(event `self.ReceiveBeginPlay`
  (bind _returnvalue (`Actor.GetComponentByClass` (`self.GetOwner`) "/Game/Blueprints/Abilities/BP_AbilityControl.BP_AbilityControl_C"))
  (`parent.ReceiveBeginPlay`)
  (`/Engine/EditorBlueprintResources/StandardMacros.IsValid` _returnvalue
    (:`Is Valid`
      (set `self.AbilityControl` _returnvalue)
      (`self.SelectBehaviour`))))

(event `self.ReceiveTick`
  (params (DeltaSeconds :type "Float (single-precision)"))
  (`parent.ReceiveTick` DeltaSeconds))

(event `SelectBehaviour`
  (bind _abilitycontrol (`self.AbilityControl`))
  (if (<= (`Actor.GetDistanceTo` (`self.GetOwner`) (`GameplayStatics.GetPlayerPawn` 0)) 150.0)
    (`/Engine/EditorBlueprintResources/StandardMacros.IsValid` (`Actor.GetComponentByClass` (`self.GetOwner`) "/Game/Blueprints/Abilities/Enemies/BPC_EnemyAttackCooldown.BPC_EnemyAttackCooldown_C")
      (:`Is Valid`
        (`/Game/Blueprints/Abilities/BP_AbilityControl.SetNextAbility` _abilitycontrol (`self.FollowComponent`) :!label _label))
      (:`Is Not Valid`
        (`/Game/Blueprints/Abilities/BP_AbilityControl.SetNextAbility` _abilitycontrol (`self.AttackComponent`))))
    (else
      (goto _label))))