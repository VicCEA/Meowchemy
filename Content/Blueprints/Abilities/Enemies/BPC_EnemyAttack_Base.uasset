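; Base enemy attack ability component for BPZD_Enemy, which plays a short attack state aimed at the player.
; On BeginPlay it sets IsAttack on the simple slime anim instance, reveals the enemy's Disc and rotates it toward the player on the horizontal plane.
; A half-second timer then clears the flag, hides the Disc and has BPAbilityControl switch to BPC_EnemySelectBehavior.
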(event `self.ReceiveBeginPlay`
  (bind _as_bpzd_enemy (`self.As BPZD Enemy`))
  (`parent.ReceiveBeginPlay`)
  (bind _asbpzd_enemy (cast `/Game/Blueprints/AI/Enemies/BPZD_Enemy` (`self.GetOwner`)))
  (set `self.As BPZD Enemy` _asbpzd_enemy)
  (bind _aszdanim_bp_simple_slime_enemy (cast `/Game/Paper2D/SlimeEnemy/ZDAnimBP_SimpleSlimeEnemy` (`PaperZDCharacter.GetAnimInstance` (`self.As BPZD Enemy`))))
  (bind _output_get (set `self.As ZDAnim BP Simple Slime Enemy` _aszdanim_bp_simple_slime_enemy))
  (set `/Game/Paper2D/SlimeEnemy/ZDAnimBP_SimpleSlimeEnemy.IsAttack` true _output_get)
  (`SceneComponent.SetHiddenInGame` (`/Game/Blueprints/AI/Enemies/BPZD_Enemy.Disc` _as_bpzd_enemy) false false)
  (`/Game/Blueprints/AI/Enemies/BPZD_Enemy.RotateDisc` _as_bpzd_enemy (`KismetMathLibrary.MakeVector` (.x (`KismetMathLibrary.Normal` (- (`Actor.K2_GetActorLocation` (`GameplayStatics.GetPlayerCharacter` 0)) (`Actor.K2_GetActorLocation` (`self.GetOwner`))))) (.y (`KismetMathLibrary.Normal` (- (`Actor.K2_GetActorLocation` (`GameplayStatics.GetPlayerCharacter` 0)) (`Actor.K2_GetActorLocation` (`self.GetOwner`)))))))
  (`KismetSystemLibrary.K2_SetTimerDelegate` (delegate `self.RemoveComponent`) 0.5))

(event `self.RemoveComponent`
  (set `/Game/Paper2D/SlimeEnemy/ZDAnimBP_SimpleSlimeEnemy.IsAttack` false (`self.As ZDAnim BP Simple Slime Enemy`))
  (`SceneComponent.SetHiddenInGame` (`/Game/Blueprints/AI/Enemies/BPZD_Enemy.Disc` (`self.As BPZD Enemy`)) true false)
  (`/Game/Blueprints/Abilities/BP_AbilityControl.SetNextAbility` (`/Game/Blueprints/AI/Enemies/BPZD_Enemy.BP_AbilityControl` (`self.As BPZD Enemy`)) "/Game/Blueprints/Abilities/Enemies/BPC_EnemySelectBehavior.BPC_EnemySelectBehavior_C"))