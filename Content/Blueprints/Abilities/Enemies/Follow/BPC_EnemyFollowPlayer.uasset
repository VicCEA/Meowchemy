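; Enemy ability component that makes its owning BPZD_Enemy chase the player pawn.
; On BeginPlay it resets the enemy's walk speed and starts an AI MoveTo toward the player.
; When the move succeeds, it sets the attack component as BP_AbilityControl's next ability, then ends itself.
; A distance-based stop-and-attack check remains in the graph but never runs.
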(event `self.ReceiveBeginPlay`
  (`parent.ReceiveBeginPlay`)
  (bind _asbpzd_enemy (cast `/Game/Blueprints/AI/Enemies/BPZD_Enemy` (`self.GetOwner`)))
  (`/Game/Blueprints/AI/Enemies/BPZD_Enemy.ResetWalkSpeed` _asbpzd_enemy)
  (`self.GoToPlayer`))

(event `self.ReceiveTick`
  (params (DeltaSeconds :type "Float (single-precision)"))
  (`parent.ReceiveTick` DeltaSeconds))

(event `GoToPlayer`
  (`|AIMoveTo` (`AIBlueprintHelperLibrary.GetAIController` (`self.GetOwner`)) null (0.0 0.0 0.0) (`GameplayStatics.GetPlayerPawn` 0) (`self.Acceptance Radius`) true
    (:`OnSuccess`
      (`self.OnMoveSuccess`))))

(event `OnMoveSuccess`
  (`self.RemoveComponent`))

(event `self.RemoveComponent`
  (bind _returnvalue (`Actor.GetComponentByClass` (`self.GetOwner`) "/Game/Blueprints/Abilities/BP_AbilityControl.BP_AbilityControl_C"))
  (`/Engine/EditorBlueprintResources/StandardMacros.IsValid` _returnvalue
    (:`Is Valid`
      (set `/Game/Blueprints/Abilities/BP_AbilityControl.NextAbility` (`self.AttackComponent`) _returnvalue)
      (`self.EndAbility`))))

(event `StopFollow`
  (`Controller.StopMovement` (`AIBlueprintHelperLibrary.GetAIController` (`self.GetOwner`))))

(fn `CheckDistance`
  (returns (InDistance :type Boolean))
  (return (<= (`Actor.GetDistanceTo` (`self.GetOwner`) (`GameplayStatics.GetPlayerPawn` 0)) (`self.AttackDistance`))))