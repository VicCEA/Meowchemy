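; Enemy hurt ability component that plays a damage reaction on a PaperZD enemy when it begins play.
; It zeroes walk speed, tints the sprite dark red, sets IsHurt on the slime AnimBP and destroys the damage component's collider.
; A clearable timer then ends the hurt state, restoring damageability and sprite color and asking BP_AbilityControl, if present, to set the next ability.
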(event `self.ReceiveBeginPlay`
  (`parent.ReceiveBeginPlay`)
  (bind _asbpzd_enemy (cast `/Game/Blueprints/AI/Enemies/BPZD_Enemy` (`self.GetOwner`)))
  (bind _output_get (set `self.As BPZD Enemy` _asbpzd_enemy))
  (set `CharacterMovementComponent.MaxWalkSpeed` 0.0 (`Character.CharacterMovement` _output_get))
  (`self.PlayAnimation`)
  (bind _returnvalue (`KismetSystemLibrary.K2_SetTimerDelegate` (delegate `EndHurt`) 1.25))
  (set `self.Timer` _returnvalue))

(event `EndHurt`
  (bind _returnvalue (`self.GetOwner`))
  (bind _returnvalue_2 (`Actor.GetComponentByClass` _returnvalue "/Game/Blueprints/Abilities/BP_AbilityControl.BP_AbilityControl_C"))
  (`self.SetHurt` false)
  (set `Actor.bCanBeDamaged` true _returnvalue)
  (`PaperFlipbookComponent.SetSpriteColor` (`PaperCharacter.Sprite` (`self.As BPZD Enemy`)) (struct :`R` 1.0 :`G` 1.0 :`B` 1.0 :`A` 1.0))
  (`/Engine/EditorBlueprintResources/StandardMacros.IsValid` _returnvalue_2
    (:`Is Valid`
      (`/Game/Blueprints/Abilities/BP_AbilityControl.SetNextAbility` _returnvalue_2 (`self.SelectComponent`)))))

(event `ResetTimer`
  (`KismetSystemLibrary.K2_ClearAndInvalidateTimerHandle` (`self.Timer`)))

(event `SetHurt`
  (params (IsHurt :type Boolean))
  (bind _aszdanim_bp_simple_slime_enemy (cast `/Game/Paper2D/SlimeEnemy/ZDAnimBP_SimpleSlimeEnemy` (`PaperZDCharacter.GetAnimInstance` (`self.As BPZD Enemy`))))
  (set `/Game/Paper2D/SlimeEnemy/ZDAnimBP_SimpleSlimeEnemy.IsHurt` IsHurt _aszdanim_bp_simple_slime_enemy))

(event `self.PlayAnimation`
  (bind _collider (`/Game/Blueprints/DamageControl/BP_DamageComponent.Collider` (`/Game/Blueprints/AI/Enemies/BPZD_Enemy.BP_DamageComponent` (`self.As BPZD Enemy`))))
  (`PaperFlipbookComponent.SetSpriteColor` (`PaperCharacter.Sprite` (`self.As BPZD Enemy`)) (struct :`R` 0.291667 :`B` 0.002532 :`A` 1.0))
  (`self.SetHurt` true)
  ;[1 1 1] Hide Collider
  (`/Engine/EditorBlueprintResources/StandardMacros.IsValid` _collider
    (:`Is Valid`
      (`Actor.K2_DestroyActor` _collider))))