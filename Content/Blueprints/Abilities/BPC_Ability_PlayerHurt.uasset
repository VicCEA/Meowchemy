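; Temporary ability component that puts the player character into a brief hurt state with invulnerability.
; On BeginPlay it turns off the owner's CanBeDamaged, sets IsHurt on the character's animation Blueprint and starts a short one-shot timer.
; When the timer fires, EndHurt clears the animation flag, restores damageability and removes the component, so the component's lifetime defines the hurt window.
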(event `self.ReceiveBeginPlay`
  (bind _returnvalue (`self.GetOwner`))
  (`parent.ReceiveBeginPlay`)
  (set `Actor.bCanBeDamaged` false _returnvalue)
  (bind _asbpzd_character (cast `/Game/Paper2D/BPZD_Character` _returnvalue))
  (bind _aszdanim_bp_character (cast `/Game/Paper2D/ZDAnimBP_Character` (`PaperZDCharacter.GetAnimInstance` _asbpzd_character)))
  (set `/Game/Paper2D/ZDAnimBP_Character.IsHurt` true _aszdanim_bp_character)
  (`KismetSystemLibrary.K2_SetTimerDelegate` (delegate `EndHurt`) 0.5))

(event `EndHurt`
  (bind _aszdanim_bp_character (cast `/Game/Paper2D/ZDAnimBP_Character` (`PaperZDCharacter.GetAnimInstance` (stale `self.ReceiveBeginPlay` _asbpzd_character))))
  (set `/Game/Paper2D/ZDAnimBP_Character.IsHurt` false _aszdanim_bp_character)
  (set `Actor.bCanBeDamaged` true (`self.GetOwner`))
  (`self.RemoveComponent`))