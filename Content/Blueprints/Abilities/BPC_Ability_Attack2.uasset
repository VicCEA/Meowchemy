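; BPC_Ability_Attack2 is an ability component for BPZD_Character, currently a placeholder that prints "Attack2" instead of performing attack logic.
; On BeginPlay it runs parent logic and starts a one-shot timer bound to RemoveComponent.
; When the timer fires, it casts the owner to BPZD_Character, notifies BPAbilityControl that the ability ended, then destroys itself.
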(event `self.ReceiveBeginPlay`
  (`parent.ReceiveBeginPlay`)
  (`KismetSystemLibrary.PrintString` "Attack2")
  (`KismetSystemLibrary.K2_SetTimerDelegate` (delegate `self.RemoveComponent`) 1.0))

(event `self.ReceiveTick`
  (params (DeltaSeconds :type "Float (single-precision)"))
  (`parent.ReceiveTick` DeltaSeconds))

(event `self.RemoveComponent`
  (bind _asbpzd_character (cast `/Game/Paper2D/BPZD_Character` (`self.GetOwner`)))
  (`/Game/Blueprints/Abilities/BP_AbilityControl.OnAbilityEnd` (`/Game/Paper2D/BPZD_Character.BP_AbilityControl` _asbpzd_character))
  (`self.K2_DestroyComponent`))