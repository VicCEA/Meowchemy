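; Player component that turns Enhanced Input actions into combo attacks, dashes, healing and companion skills.
; Attacks and dashes are buffered through BP_AbilityControl, with the current ability choosing the next of three combo steps.
; Special attacks spend tiered Ghost Power, then send the companion to the nearest enemy with a possession skill.
; Holding heal restores health by held time, locking movement and playing a sound until release.
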(event `self.ReceiveBeginPlay`
  (`self.CheckPlayerReference`))

(event `EnhancedInput|/Game/Input/IA_Attack`
  (params (ActionValue :type Boolean) (ElapsedSeconds :type "Float (double-precision)") (TriggeredSeconds :type "Float (double-precision)") (InputAction :type "InputAction Object Reference" :default "/Game/Input/IA_Attack.IA_Attack"))
  (:`Started`
    (bind _output_get (`self.CheckPlayerReference`))
    (if (`Actor.bCanBeDamaged` _output_get)
      (if (not (`self.IsHealing`))
        (`self.ComboAttacks`)))))

(event `EnhancedInput|/Game/Input/IA_Dash`
  (params (ActionValue :type Boolean) (ElapsedSeconds :type "Float (double-precision)") (TriggeredSeconds :type "Float (double-precision)") (InputAction :type "InputAction Object Reference" :default "/Game/Input/IA_Dash.IA_Dash"))
  (:`Started`
    (`self.CheckPlayerReference`)
    (if (not (`self.IsHealing`))
      (`self.Dash`))))

(event `EnhancedInput|/Game/Input/IA_SpecialAttack1`
  (params (ActionValue :type Boolean) (ElapsedSeconds :type "Float (double-precision)") (TriggeredSeconds :type "Float (double-precision)") (InputAction :type "InputAction Object Reference" :default "/Game/Input/IA_SpecialAttack1.IA_SpecialAttack1"))
  (:`Started`
    (bind _drained (`self.DrainPower` 1.0))
    (if _drained
      (`self.AddSkillToCompanion` "/Game/Blueprints/Abilities/Companion/BPC_CompanionPosses_Skill.BPC_CompanionPosses_Skill_C"))))

(event `EnhancedInput|/Game/Input/IA_SpecialAttack2`
  (params (ActionValue :type Boolean) (ElapsedSeconds :type "Float (double-precision)") (TriggeredSeconds :type "Float (double-precision)") (InputAction :type "InputAction Object Reference" :default "/Game/Input/IA_SpecialAttack2.IA_SpecialAttack2"))
  (:`Started`
    (bind _drained (`self.DrainPower` 2.0))
    (if _drained
      (`self.AddSkillToCompanion` "/Game/Blueprints/Abilities/Companion/BPC_CompanionPosses_SkillExplode.BPC_CompanionPosses_SkillExplode_C"))))

(event `EnhancedInput|/Game/Input/IA_SpecialAttack3`
  (params (ActionValue :type Boolean) (ElapsedSeconds :type "Float (double-precision)") (TriggeredSeconds :type "Float (double-precision)") (InputAction :type "InputAction Object Reference" :default "/Game/Input/IA_SpecialAttack3.IA_SpecialAttack3"))
  (:`Started`
    (bind _drained (`self.DrainPower` 3.0))
    (if _drained
      (`self.AddSkillToCompanion` "/Game/Blueprints/Abilities/Companion/BPC_CompanionPosses_SkillVortex.BPC_CompanionPosses_SkillVortex_C"))))

(event `EnhancedInput|/Game/Input/IA_Heal`
  (params (ActionValue :type Boolean) (ElapsedSeconds :type "Float (double-precision)") (TriggeredSeconds :type "Float (double-precision)") (InputAction :type "InputAction Object Reference" :default "/Game/Input/IA_Heal.IA_Heal"))
  (:`Triggered`
    (bind _output_get (`self.CheckPlayerReference`))
    (if (`Actor.bCanBeDamaged` _output_get)
      (if (not (`/Game/Blueprints/Abilities/BP_AbilityControl.CheckForAbility` (`self.AbilityControl`)))
        (`self.HealPlayer` TriggeredSeconds)
        (`/Engine/EditorBlueprintResources/StandardMacros.DoOnce` false :!label _label
          (:`Completed`
            (`/Engine/EditorBlueprintResources/StandardMacros.IsValid` (`self.HealSound`)
              (:`Is Valid`
                _)
              (:`Is Not Valid`
                (bind _returnvalue (`GameplayStatics.SpawnSound2D` "/Game/Sounds/Meowko/341547__nakhas__cat-grooming.341547__nakhas__cat-grooming" 2.0 1.0 0.0 null))
                (set `self.HealSound` _returnvalue)))
            (`AudioComponent.Play` (`self.HealSound`) 0.0))))))
  (:`Completed`
    (set `self.IsHealing` false)
    (`Controller.ResetIgnoreMoveInput` (`GameplayStatics.GetPlayerController` 0))
    (`AudioComponent.Stop` (`self.HealSound`))
    (goto _label :!via `Reset`)))

(event `AddSkillToCompanion`
  (params (NextAbility :type "ActorComponent Class Reference"))
  (bind _as_bpzd_character (`self.As BPZD Character`))
  (bind (_normalizeddirection _enemyvalid _nearestenemyref) (`/Game/Paper2D/BPZD_Character.GetNearestEnemy` _as_bpzd_character))
  (if _enemyvalid
    (`/Game/Blueprints/AI/Companion/BPZD_Companion.GoToLocation` (`/Game/Paper2D/BPZD_Character.CompanionRef` _as_bpzd_character) (`Actor.K2_GetActorLocation` _nearestenemyref) NextAbility)))

(fn `CheckPlayerReference`
  (returns (Output_Get :type "/Game/Paper2D/BPZD_Character Object Reference"))
  (`/Engine/EditorBlueprintResources/StandardMacros.IsValid` (`self.As BPZD Character`)
    (:`Is Valid`
      _)
    (:`Is Not Valid`
      (bind _asbpzd_character (cast `/Game/Paper2D/BPZD_Character` (`Controller.K2_GetPawn` (`GameplayStatics.GetPlayerController` 0))))
      (set `self.As BPZD Character` _asbpzd_character)
      (bind _returnvalue (`Actor.GetComponentByClass` _asbpzd_character "/Game/Blueprints/Abilities/BP_AbilityControl.BP_AbilityControl_C"))
      (`/Engine/EditorBlueprintResources/StandardMacros.IsValid` _returnvalue
        (:`Is Valid`
          (set `self.AbilityControl` _returnvalue)))))
  (return (`self.As BPZD Character`)))

(fn `ComboAttacks`
  (bind _abilitycontrol (`self.AbilityControl`))
  (if (`/Game/Blueprints/Abilities/BP_AbilityControl.CheckForAbility` _abilitycontrol)
    (if (== (`/Game/Blueprints/Abilities/BP_AbilityControl.CurrentAbility` (`self.AbilityControl`)) "/Game/Blueprints/Abilities/Player/Attacks/BPC_Ability_Attack1.BPC_Ability_Attack1_C")
      (`/Game/Blueprints/Abilities/BP_AbilityControl.BufferNextAbility` _abilitycontrol "/Game/Blueprints/Abilities/Player/Attacks/BPC_Ability_Attack2.BPC_Ability_Attack2_C")
      (elif (== (`/Game/Blueprints/Abilities/BP_AbilityControl.CurrentAbility` _abilitycontrol) "/Game/Blueprints/Abilities/Player/Attacks/BPC_Ability_Attack2.BPC_Ability_Attack2_C")
        (`/Game/Blueprints/Abilities/BP_AbilityControl.BufferNextAbility` (`self.AbilityControl`) "/Game/Blueprints/Abilities/Player/Attacks/BPC_Ability_Attack3.BPC_Ability_Attack3_C")))
    (else
      (`/Game/Blueprints/Abilities/BP_AbilityControl.BufferNextAbility` _abilitycontrol "/Game/Blueprints/Abilities/Player/Attacks/BPC_Ability_Attack1.BPC_Ability_Attack1_C"))))

(fn `Dash`
  (if (not (`NavMovementComponent.IsFalling` (`Character.CharacterMovement` (`self.As BPZD Character`))))
    (`/Game/Blueprints/Abilities/BP_AbilityControl.BufferNextAbility` (`self.AbilityControl`) "/Game/Blueprints/Abilities/Player/BPC_Ability_Dash.BPC_Ability_Dash_C")))

(fn `DrainPower`
  (params (Value :type "Float (double-precision)"))
  (returns (Drained :type Boolean))
  (bind _returnvalue (`Actor.GetComponentByClass` (`self.GetOwner`) "/Game/Blueprints/Abilities/Stats/BPC_FVS_GhostPower.BPC_FVS_GhostPower_C"))
  (`/Engine/EditorBlueprintResources/StandardMacros.IsValid` _returnvalue
    (:`Is Valid`
      (if (>= (`/Game/Blueprints/Abilities/Stats/BPC_FloatValueSystem.CurrentValue` _returnvalue) Value)
        (`/Game/Blueprints/Abilities/Stats/BPC_FloatValueSystem.DecreaseValue` _returnvalue Value)
        (return true)
        (else
          (return false))))))

(fn `HealPlayer`
  (params (A :type "Float (double-precision)"))
  (set `self.IsHealing` true)
  (`Controller.SetIgnoreMoveInput` (`GameplayStatics.GetPlayerController` 0) true)
  (`/Game/Blueprints/Abilities/Stats/BPC_FloatValueSystem.IncreaseVlaue` (`/Game/Paper2D/BPZD_Character.BPC_FVS_Health` (`self.As BPZD Character`)) (* A 0.1)))