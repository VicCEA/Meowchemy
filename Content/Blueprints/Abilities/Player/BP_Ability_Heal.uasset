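; Player heal ability that blocks movement input and restores health to the owning BPZD_Character.
; On BeginPlay it disables move input on player controller 0, then caches the owner's BPCFVSHealth reference.
; Each Tick adds a fixed amount to that health without scaling by delta time, so healing depends on frame rate.
; This graph never re-enables move input or stops the healing.
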(event `self.ReceiveBeginPlay`
  (`parent.ReceiveBeginPlay`)
  (`Controller.SetIgnoreMoveInput` (`GameplayStatics.GetPlayerController` 0) true)
  (bind _asbpzd_character (cast `/Game/Paper2D/BPZD_Character` (`self.GetOwner`)))
  (set `self.BPC FVS Health` (`/Game/Paper2D/BPZD_Character.BPC_FVS_Health` _asbpzd_character)))

(event `self.ReceiveTick`
  (params (DeltaSeconds :type "Float (single-precision)"))
  (`parent.ReceiveTick` DeltaSeconds)
  (`/Game/Blueprints/Abilities/Stats/BPC_FloatValueSystem.IncreaseVlaue` (`self.BPC FVS Health`) 10.0))