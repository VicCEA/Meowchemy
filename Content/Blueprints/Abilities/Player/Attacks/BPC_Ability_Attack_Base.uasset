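; Base ability component for player attacks that plays an indexed PaperZD attack animation while lunging the character at the nearest enemy.
; On BeginPlay it stops movement, sets AnimBP attack flags and shows the character's disc.
; A sphere overlap picks the closest enemy to set facing, launch and disc direction, falling back to move direction.
; A flipbook-length timer restores movement, clears flags, hides the disc and notifies ability control.
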(event `self.ReceiveBeginPlay`
  (`parent.ReceiveBeginPlay`)
  (`self.StopMovement`)
  (bind _asbpzd_character (cast `/Game/Paper2D/BPZD_Character` (`self.GetOwner`)))
  (set `self.As BPZD Character` _asbpzd_character)
  (`self.PlayAnimation`)
  (`self.ApplyEffect`)
  (`KismetSystemLibrary.K2_SetTimerDelegate` (delegate `self.RemoveComponent`) (`/Game/Blueprints/FL_Utilities.CalculateFlipbookDuration` (`self.AnimationFrames`))))

(event `self.ReceiveTick`
  (params (DeltaSeconds :type "Float (single-precision)"))
  (`parent.ReceiveTick` DeltaSeconds))

(event `self.RemoveComponent`
  (`self.ResetMovement`)
  (`self.StopAnimation`)
  (`/Game/Paper2D/BPZD_Character.HideDisc` (`self.As BPZD Character`) true)
  (`/Game/Blueprints/Abilities/BP_AbilityControl.OnAbilityEnd` (`/Game/Paper2D/BPZD_Character.BP_AbilityControl` (`self.As BPZD Character`))))

(event `self.PlayAnimation`
  (bind _aszdanim_bp_character (cast `/Game/Paper2D/ZDAnimBP_Character` (`PaperZDCharacter.GetAnimInstance` (`self.As BPZD Character`))))
  (set `/Game/Paper2D/ZDAnimBP_Character.IsAbliity` true _aszdanim_bp_character)
  (set `/Game/Paper2D/ZDAnimBP_Character.IsAttack` true _aszdanim_bp_character)
  (set `/Game/Paper2D/ZDAnimBP_Character.AttackIndex` (`self.AttackIndex`) _aszdanim_bp_character))

(event `self.StopAnimation`
  (bind _aszdanim_bp_character (cast `/Game/Paper2D/ZDAnimBP_Character` (`PaperZDCharacter.GetAnimInstance` (`self.As BPZD Character`))))
  (set `/Game/Paper2D/ZDAnimBP_Character.IsAbliity` false _aszdanim_bp_character)
  (set `/Game/Paper2D/ZDAnimBP_Character.IsAttack` false _aszdanim_bp_character))

(event `self.ApplyEffect`
  (`/Game/Paper2D/BPZD_Character.HideDisc` (`self.As BPZD Character`) false)
  (`MovementComponent.StopMovementImmediately` (`Character.CharacterMovement` (`self.As BPZD Character`)))
  (`self.GetNearestEnemy`))

(event `GetNearestEnemy`
  (bind _as_bpzd_character (`self.As BPZD Character`))
  (bind _nearestenemy (`self.NearestEnemy`))
  (bind _as_bpzd_character_2 (`self.As BPZD Character`))
  (bind _as_bpzd_character_3 (`self.As BPZD Character`))
  (bind _normalizeddirection (`/Game/Blueprints/FL_Utilities.CalculateDirectionBetweenTwoActors` (`self.NearestEnemy`) (`self.As BPZD Character`)))
  (bind _movedirection (`/Game/Paper2D/BPZD_Character.MoveDirection` _as_bpzd_character_3))
  (bind (_returnvalue_roll _returnvalue_pitch _returnvalue_yaw) (`KismetMathLibrary.BreakRotator` (`KismetMathLibrary.MakeRotFromX` (`KismetMathLibrary.MakeVector` (.x _normalizeddirection) (.y _normalizeddirection)))))
  (bind _outactors (`KismetSystemLibrary.SphereOverlapActors` (`Actor.K2_GetActorLocation` _as_bpzd_character_2) 2000.0 (`|MakeArray` "ObjectTypeQuery3" :!type "EObjectTypeQuery Enum") "/Game/Blueprints/AI/Enemies/BPZD_Enemy.BPZD_Enemy_C" (`|MakeArray` _as_bpzd_character_2 :!type "Actor Object Reference")))
  (for _array_element _outactors
    (`/Engine/EditorBlueprintResources/StandardMacros.IsValid` _nearestenemy
      (:`Is Valid`
        (if (< (`Actor.GetDistanceTo` _as_bpzd_character _array_element) (`Actor.GetDistanceTo` _as_bpzd_character _nearestenemy))
          (set `self.NearestEnemy` _array_element)))
      (:`Is Not Valid`
        (set `self.NearestEnemy` _array_element))))
  (`/Engine/EditorBlueprintResources/StandardMacros.IsValid` (`self.NearestEnemy`)
    (:`Is Valid`
      (`/Game/Paper2D/BPZD_Character.UpdateControlRotation` _as_bpzd_character_3 _returnvalue_yaw)
      (`Character.LaunchCharacter` _as_bpzd_character_3 (* _normalizeddirection 1500.0) true false)
      (`/Game/Paper2D/BPZD_Character.RotateDisc` (`self.As BPZD Character`) _normalizeddirection))
    (:`Is Not Valid`
      (`Character.LaunchCharacter` _as_bpzd_character_3 (* _movedirection 1500.0) true false)
      (`/Game/Paper2D/BPZD_Character.RotateDisc` (`self.As BPZD Character`) _movedirection))))