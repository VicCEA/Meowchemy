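; Base component for player special attacks, running one timed ability on the owning BPZD_Character.
; On BeginPlay it stops the character's movement, toggles the disc via HideDisc, sets the anim Blueprint's ability, special and attack-index variables, and starts a timer.
; When the timer fires, it clears the animation flags, toggles the disc back and notifies BPAbilityControl that the ability ended.
; ApplyEffect is an empty event, and Tick is disabled.
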(event `self.ReceiveBeginPlay`
  (`parent.ReceiveBeginPlay`)
  (bind _asbpzd_character (cast `/Game/Paper2D/BPZD_Character` (`self.GetOwner`)))
  (set `self.As BPZD Character` _asbpzd_character)
  (`self.PlayAnimation`)
  (`KismetSystemLibrary.K2_SetTimerDelegate` (delegate `self.RemoveComponent`) (`self.Time`))
  (`/Game/Paper2D/BPZD_Character.HideDisc` (`self.As BPZD Character`) false)
  (`MovementComponent.StopMovementImmediately` (`Character.CharacterMovement` (`self.As BPZD Character`))))

(event `self.RemoveComponent`
  (`self.StopAnimation`)
  (`/Game/Paper2D/BPZD_Character.HideDisc` (`self.As BPZD Character`) true)
  (`/Game/Blueprints/Abilities/BP_AbilityControl.OnAbilityEnd` (`/Game/Paper2D/BPZD_Character.BP_AbilityControl` (`self.As BPZD Character`))))

(event `self.PlayAnimation`
  (bind _aszdanim_bp_character (cast `/Game/Paper2D/ZDAnimBP_Character` (`PaperZDCharacter.GetAnimInstance` (`self.As BPZD Character`))))
  (set `/Game/Paper2D/ZDAnimBP_Character.IsAbliity` true _aszdanim_bp_character)
  (set `/Game/Paper2D/ZDAnimBP_Character.IsSpecial` true _aszdanim_bp_character)
  (set `/Game/Paper2D/ZDAnimBP_Character.AttackIndex` (`self.Attack Index`) _aszdanim_bp_character))

(event `self.StopAnimation`
  (bind _aszdanim_bp_character (cast `/Game/Paper2D/ZDAnimBP_Character` (`PaperZDCharacter.GetAnimInstance` (`self.As BPZD Character`))))
  (set `/Game/Paper2D/ZDAnimBP_Character.IsAbliity` false _aszdanim_bp_character)
  (set `/Game/Paper2D/ZDAnimBP_Character.IsSpecial` false _aszdanim_bp_character))

(event `self.ApplyEffect`)