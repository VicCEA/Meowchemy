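; Player dash ability component for the PaperZD character that starts as soon as it begins play.
; It makes the owner invulnerable, applies a velocity-change impulse along its move direction, enlarges the sprite and sets the dash flags on its animation instance.
; A short timer then restores damage, sprite scale and flags, and notifies the owner's ability control that the ability ended.
; An alternative LaunchCharacter path is left disconnected.
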(event `self.ReceiveBeginPlay`
  (`parent.ReceiveBeginPlay`)
  (`self.ApplyEffect`))

(event `self.ReceiveTick`
  (params (DeltaSeconds :type "Float (single-precision)"))
  (`parent.ReceiveTick` DeltaSeconds))

(event `self.ApplyEffect`
  (bind _asbpzd_character (cast `/Game/Paper2D/BPZD_Character` (`self.GetOwner`)))
  (set `Actor.bCanBeDamaged` false _asbpzd_character)
  (`self.PlayAnimation`)
  (`CharacterMovementComponent.AddImpulse` (`Character.CharacterMovement` _asbpzd_character) (* (`KismetMathLibrary.Normal` (`/Game/Paper2D/BPZD_Character.MoveDirection` _asbpzd_character)) (`self.DashDistance`)) true)
  (`KismetSystemLibrary.K2_SetTimerDelegate` (delegate `self.RemoveComponent`) 0.6))

(event `self.RemoveComponent`
  (set `Actor.bCanBeDamaged` true (`self.GetOwner`))
  (bind _asbpzd_character (cast `/Game/Paper2D/BPZD_Character` (`self.GetOwner`)))
  (`self.StopAnimation`)
  (`/Game/Blueprints/Abilities/BP_AbilityControl.OnAbilityEnd` (`/Game/Paper2D/BPZD_Character.BP_AbilityControl` _asbpzd_character)))

(event `self.PlayAnimation`
  (bind _asbpzd_character (cast `/Game/Paper2D/BPZD_Character` (`self.GetOwner`)))
  (`SceneComponent.SetRelativeScale3D` (`PaperCharacter.Sprite` _asbpzd_character) (3.0 3.0 3.0))
  (bind _aszdanim_bp_character (cast `/Game/Paper2D/ZDAnimBP_Character` (`PaperZDCharacter.GetAnimInstance` _asbpzd_character)))
  (set `/Game/Paper2D/ZDAnimBP_Character.IsAbliity` true _aszdanim_bp_character)
  (set `/Game/Paper2D/ZDAnimBP_Character.IsDash` true _aszdanim_bp_character))

(event `self.StopAnimation`
  (bind _asbpzd_character (cast `/Game/Paper2D/BPZD_Character` (`self.GetOwner`)))
  (`SceneComponent.SetRelativeScale3D` (`PaperCharacter.Sprite` _asbpzd_character) (0.2 0.2 0.2))
  (bind _aszdanim_bp_character (cast `/Game/Paper2D/ZDAnimBP_Character` (`PaperZDCharacter.GetAnimInstance` _asbpzd_character)))
  (set `/Game/Paper2D/ZDAnimBP_Character.IsAbliity` false _aszdanim_bp_character)
  (set `/Game/Paper2D/ZDAnimBP_Character.IsDash` false _aszdanim_bp_character))