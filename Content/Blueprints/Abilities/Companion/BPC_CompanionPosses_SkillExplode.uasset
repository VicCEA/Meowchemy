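; Companion possession skill component for the explode variant, extending a parent skill component that handles begin play, tick and removal.
; Applying the skill sets the enemy's next ability to BPC_EnemyExplode through its ability control.
; Its effect step runs a fixed-radius sphere overlap.
; On removal it spawns an enlarged poof Niagara effect at the possess location before calling the parent removal.
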(event `self.ReceiveBeginPlay`
  (`parent.ReceiveBeginPlay`))

(event `self.ReceiveTick`
  (params (DeltaSeconds :type "Float (single-precision)"))
  (`parent.ReceiveTick` DeltaSeconds))

(event `self.ApplySkill`
  (params (Enemy :type "/Game/Blueprints/AI/Enemies/BPZD_Enemy Object Reference"))
  (`/Game/Blueprints/Abilities/BP_AbilityControl.SetNextAbility` (`/Game/Blueprints/AI/Enemies/BPZD_Enemy.BP_AbilityControl` Enemy) "/Game/Blueprints/Abilities/Enemies/BPC_EnemyExplode.BPC_EnemyExplode_C"))

(event `/Game/Blueprints/Abilities/BPC_Ability_Base.ApplyEffect`
  (`self.OverlapSphere` 600.0))

(event `/Game/Blueprints/Abilities/BPC_Ability_Base.RemoveComponent`
  (`NiagaraFunctionLibrary.SpawnSystemAtLocation` "/Game/Assets/Vfx/N_Poof.N_Poof" (`self.Possess Location`) (struct) (4.0 4.0 4.0))
  (`parent.RemoveComponent`))