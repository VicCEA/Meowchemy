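; Companion follow component that makes its owner trail the player's BPZD_Character.
; It caches the player character on BeginPlay, retrying on Tick while invalid, and unhides the owner at start.
; Each tick it eases the owner toward the character's CompanionLocation with a lerp scaled by delta time and Speed.
; Facing snaps along the Y axis toward that point, with a fixed default rotation when the Y direction is zero.
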(event `self.ReceiveBeginPlay`
  (`parent.ReceiveBeginPlay`)
  (`self.GetPlayer`)
  (`Actor.SetActorHiddenInGame` (`self.GetOwner`) false))

(event `self.ReceiveTick`
  (params (DeltaSeconds :type "Float (single-precision)"))
  (`parent.ReceiveTick` DeltaSeconds)
  (`/Engine/EditorBlueprintResources/StandardMacros.IsValid` (`self.As BPZD Character`)
    (:`Is Valid`
      _)
    (:`Is Not Valid`
      (`self.GetPlayer`)))
  (`self.SetCompanionLocation` DeltaSeconds))

(event `GetPlayer`
  (bind _asbpzd_character (cast `/Game/Paper2D/BPZD_Character` (`GameplayStatics.GetPlayerCharacter` 0)))
  (set `self.As BPZD Character` _asbpzd_character))

(event `SetCompanionLocation`
  (params (A :type "Float (double-precision)"))
  (bind _returnvalue (`self.GetOwner`))
  (bind _returnvalue_2 (`Actor.K2_GetActorLocation` _returnvalue))
  (bind _returnvalue_3 (`SceneComponent.K2_GetComponentLocation` (`/Game/Paper2D/BPZD_Character.CompanionLocation` (`self.As BPZD Character`))))
  (bind (_normalizeddirection_x _normalizeddirection_y) (`KismetMathLibrary.BreakVector` (`/Game/Blueprints/FL_Utilities.CalculateDirectionBetweenTwoLocations` _returnvalue_2 _returnvalue_3)))
  (if (!= _normalizeddirection_y 0.0)
    (`Actor.K2_SetActorRotation` _returnvalue (`KismetMathLibrary.Conv_VectorToRotator` (`KismetMathLibrary.MakeVector` 0.0 _normalizeddirection_y)) true)
    (else
      (`Actor.K2_SetActorRotation` _returnvalue (struct :`Yaw` 90.0) true)))
  (`Actor.K2_SetActorLocation` _returnvalue (`KismetMathLibrary.VLerp` _returnvalue_2 _returnvalue_3 (* A (`self.Speed`))) false false))