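; Companion possess skill component that puts a hold on enemies clustered around the enemy nearest the player.
; BeginPlay caches that enemy's location, or begins removal if none is valid.
; ApplyEffect runs a sphere overlap there, adding BPC_EnemyHold to enemies lacking it and clearing their current ability.
; RemoveComponent, despite its name, only waits briefly, then calls StopDirected on the owning companion.
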(event `self.ReceiveBeginPlay`
  (bind _asbpzd_character (cast `/Game/Paper2D/BPZD_Character` (`GameplayStatics.GetPlayerCharacter` 0)))
  (bind (_normalizeddirection _enemyvalid _nearestenemyref) (`/Game/Paper2D/BPZD_Character.GetNearestEnemy` _asbpzd_character))
  (if _enemyvalid
    (set `self.Nearest Enemy Ref` _nearestenemyref)
    (set `self.Possess Location` (`Actor.K2_GetActorLocation` _nearestenemyref))
    (set `self.Enemy Valid` _enemyvalid)
    (else
      (`self.SetComponentTickEnabled` false)
      (`self.RemoveComponent`))))

(event `self.ReceiveTick`
  (params (DeltaSeconds :type "Float (single-precision)"))
  (`parent.ReceiveTick` DeltaSeconds))

(event `self.ApplyEffect`
  (`self.OverlapSphere` 500.0))

(event `self.RemoveComponent`
  (`KismetSystemLibrary.Delay` 1.0)
  (bind _asbpzd_companion (cast `/Game/Blueprints/AI/Companion/BPZD_Companion` (`self.GetOwner`)))
  (`/Game/Blueprints/AI/Companion/BPZD_Companion.StopDirected` _asbpzd_companion))

(event `ApplySkill`
  (params (Enemy :type "/Game/Blueprints/AI/Enemies/BPZD_Enemy Object Reference"))
  (`/Engine/EditorBlueprintResources/StandardMacros.IsValid` (`Actor.GetComponentByClass` Enemy "/Game/Blueprints/Abilities/Enemies/BPC_EnemyHold.BPC_EnemyHold_C")
    (:`Is Not Valid`
      (`|AddComponentByClass` Enemy "/Game/Blueprints/Abilities/Enemies/BPC_EnemyHold.BPC_EnemyHold_C")
      (set `/Game/Blueprints/Abilities/BP_AbilityControl.CurrentAbility` null (`/Game/Blueprints/AI/Enemies/BPZD_Enemy.BP_AbilityControl` Enemy)))))

(event `OverlapSphere`
  (params (SphereRadius :type "Float (single-precision)" :default 500.0))
  (bind _outactors (`KismetSystemLibrary.SphereOverlapActors` (`self.Possess Location`) SphereRadius (`|MakeArray` "ObjectTypeQuery7" :!type "EObjectTypeQuery Enum") "/Script/Engine.Actor" (`|MakeArray` (`self.GetOwner`) (`GameplayStatics.GetPlayerPawn` 0) :!type "Actor Object Reference")))
  (for _array_element _outactors
    (bind _asbpzd_enemy (cast `/Game/Blueprints/AI/Enemies/BPZD_Enemy` _array_element))
    (`self.ApplySkill` _asbpzd_enemy))
  (`self.RemoveComponent`))