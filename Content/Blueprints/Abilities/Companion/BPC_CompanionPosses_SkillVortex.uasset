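; Companion possession skill component for the Vortex ability, acting on the nearest enemy reference.
; ApplySkill casts that reference to BPZD_Enemy, calls ApplySkill with it and removes the component.
; ApplyEffect spawns a BP_Vortex at the enemy's transform, owned by the first player controller with its pawn as instigator, then removes the component.
; BeginPlay is unused and Tick only calls the parent.
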(event `self.ReceiveTick`
  (params (DeltaSeconds :type "Float (single-precision)"))
  (`parent.ReceiveTick` DeltaSeconds))

(event `self.ApplySkill`
  (params (Enemy :type "/Game/Blueprints/AI/Enemies/BPZD_Enemy Object Reference"))
  (bind _asbpzd_enemy (cast `/Game/Blueprints/AI/Enemies/BPZD_Enemy` (`self.Nearest Enemy Ref`)))
  (`self.ApplySkill` _asbpzd_enemy)
  (`self.RemoveComponent`))

(event `self.ApplyEffect`
  (bind _returnvalue (`GameplayStatics.GetPlayerController` 0))
  (`|SpawnActorFromClass` "/Game/Blueprints/Abilities/BP_Vortex.BP_Vortex_C" (`Actor.GetTransform` (`self.Nearest Enemy Ref`)) "Undefined" "OverrideRootScale" _returnvalue (`Controller.K2_GetPawn` _returnvalue))
  (`self.RemoveComponent`))