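; Companion component that flies its owning BPZD_Companion to a possess location to trigger a possession interaction.
; BeginPlay caches the companion's PossessLocation, and Tick eases the owner toward it with a delta-time-scaled lerp, without sweeping.
; Once within a small radius, a DoOnce hides the companion in game and calls InteractWithObjects on the player character's BPC_Interaction component.
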(event `self.ReceiveBeginPlay`
  (bind _returnvalue (`Actor.GetComponentByClass` (`GameplayStatics.GetPlayerCharacter` 0) "/Game/Blueprints/Interaction/BPC_Interaction.BPC_Interaction_C"))
  (`parent.ReceiveBeginPlay`)
  (bind _asbpzd_companion (cast `/Game/Blueprints/AI/Companion/BPZD_Companion` (`self.GetOwner`)))
  (set `self.Possess Location` (`/Game/Blueprints/AI/Companion/BPZD_Companion.PossessLocation` _asbpzd_companion))
  (goto _label :!via `Reset`))

(event `self.ReceiveTick`
  (params (DeltaSeconds :type "Float (single-precision)"))
  (bind _returnvalue (`self.GetOwner`))
  (bind _possess_location (`self.Possess Location`))
  (bind _returnvalue_2 (`Actor.K2_GetActorLocation` _returnvalue))
  (bind _returnvalue_3 (`Actor.GetComponentByClass` (`GameplayStatics.GetPlayerCharacter` 0) "/Game/Blueprints/Interaction/BPC_Interaction.BPC_Interaction_C"))
  (`parent.ReceiveTick` DeltaSeconds)
  (`Actor.K2_SetActorLocation` _returnvalue (`KismetMathLibrary.VLerp` _returnvalue_2 _possess_location (* DeltaSeconds 5.0)) false false)
  (if (<= (`KismetMathLibrary.Vector_Distance` _returnvalue_2 _possess_location) 50.0)
    (`/Engine/EditorBlueprintResources/StandardMacros.DoOnce` false :!label _label
      (:`Completed`
        (`Actor.SetActorHiddenInGame` (`self.GetOwner`) true)
        (`/Engine/EditorBlueprintResources/StandardMacros.IsValid` _returnvalue_3
          (:`Is Valid`
            (`/Game/Blueprints/Interaction/BPC_Interaction.InteractWithObjects` _returnvalue_3)))))))