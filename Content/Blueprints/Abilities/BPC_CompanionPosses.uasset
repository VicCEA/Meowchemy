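; Actor component for a companion that glides its owner to a possess location, apparently as part of a possession ability.
; On BeginPlay it casts the owner to BPZD_Companion and copies its PossessLocation once.
; Each Tick it lerps the owner's location toward that stored point by a delta-time-scaled alpha, easing in without sweep collision.
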(event `self.ReceiveBeginPlay`
  (`parent.ReceiveBeginPlay`)
  (bind _asbpzd_companion (cast `/Game/Blueprints/AI/Companion/BPZD_Companion` (`self.GetOwner`)))
  (set `self.Possess Location` (`/Game/Blueprints/AI/Companion/BPZD_Companion.PossessLocation` _asbpzd_companion)))

(event `self.ReceiveTick`
  (params (DeltaSeconds :type "Float (single-precision)"))
  (bind _returnvalue (`self.GetOwner`))
  (`parent.ReceiveTick` DeltaSeconds)
  (`Actor.K2_SetActorLocation` _returnvalue (`KismetMathLibrary.VLerp` (`Actor.K2_GetActorLocation` _returnvalue) (`self.Possess Location`) (* DeltaSeconds 5.0)) false false))