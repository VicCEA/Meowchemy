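; BP_DamageComponent is a component for PaperZD characters that creates and removes a damage collider during attacks.
; On BeginPlay it binds to the start and stop attack events of the owner's ZDAnimBP_Character, so the animation Blueprint drives the timing.
; Attack start spawns a BP_DamageCollider at the component's world transform, with the character as owner and instigator.
; Attack stop destroys that stored collider.
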(event `StopAttack`
  (`Actor.K2_DestroyActor` (`self.Collider`)))

(event `self.ReceiveBeginPlay`
  (bind _aspaper_zdcharacter (cast `PaperZDCharacter` (`self.GetOwner`)))
  (bind _output_get (set `self.As Paper ZDCharacter` _aspaper_zdcharacter))
  (bind _aszdanim_bp_character (cast `/Game/Paper2D/ZDAnimBP_Character` (`PaperZDCharacter.GetAnimInstance` _output_get)))
  (add `/Game/Paper2D/ZDAnimBP_Character.EventStartAttack` _aszdanim_bp_character (delegate `StartAttack`))
  (add `/Game/Paper2D/ZDAnimBP_Character.EventStopAttack` _aszdanim_bp_character (delegate `StopAttack`)))

(event `StartAttack`
  (bind _as_paper_zdcharacter (`self.As Paper ZDCharacter`))
  (bind _returnvalue (`|SpawnActorFromClass` "/Game/Blueprints/Abilities/DamageControl/BP_DamageCollider.BP_DamageCollider_C" (`self.K2_GetComponentToWorld`) "Undefined" "OverrideRootScale" _as_paper_zdcharacter _as_paper_zdcharacter))
  (set `self.Collider` _returnvalue))