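; BP_DialogueBox is a trigger actor that plays a one-shot dialogue when a BPZD_Character enters its box.
; Its container component supplies the lines, filled at construction when set to use a dialogue table.
; A WI_DialogueText widget, created on BeginPlay, receives them on overlap and takes UI-only input focus.
; When dialogue ends, a bound event removes the widget and destroys the actor, without restoring the input mode.
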(event `self.ReceiveBeginPlay`
  (bind _returnvalue (`|CreateWidget` "/Game/UI/WI_DialogueText.WI_DialogueText_C" (`GameplayStatics.GetPlayerController` 0)))
  (bind _output_get (set `self.Widget` _returnvalue))
  (set `/Game/UI/WI_DialogueText.DialogueBox` self _output_get))

(event `/Game/Blueprints/Dialogue/BPI_Dialogue.Talk`
  (bind _widget (`self.Widget`))
  (`KismetSystemLibrary.PrintString` "Started Dialogue")
  (`self.CreateWidget`)
  (`/Game/UI/WI_DialogueText.Filltexts` _widget (`/Game/Blueprints/Dialogue/BPC_DialogueContainer.Dialogue` (`self.BPC_DialogueContainer`)))
  (`/Game/UI/WI_DialogueText.ShowLine` _widget))

(event `self.Box.OnComponentBeginOverlap`
  (params (OverlappedComponent :type "PrimitiveComponent Object Reference") (OtherActor :type "Actor Object Reference") (OtherComp :type "PrimitiveComponent Object Reference") (OtherBodyIndex :type Integer) (bFromSweep :type Boolean) (SweepResult :type "HitResult Structure (by ref)"))
  (cast `/Game/Paper2D/BPZD_Character` OtherActor)
  (set `self.IsPlayer` true)
  (`/Game/Blueprints/Dialogue/BPI_Dialogue.Talk`)
  (`self.BindWidgetRemoval`))

(event `self.Box.OnComponentEndOverlap`
  (params (OverlappedComponent :type "PrimitiveComponent Object Reference") (OtherActor :type "Actor Object Reference") (OtherComp :type "PrimitiveComponent Object Reference") (OtherBodyIndex :type Integer))
  (cast `/Game/Paper2D/BPZD_Character` OtherActor)
  (set `self.IsPlayer` false))

(event `BindWidgetRemoval`
  (add `self.OnDialogueEnded` (delegate `RemoveWidget`)))

(event `RemoveWidget`
  (`Widget.RemoveFromParent` (`self.Widget`))
  (`KismetSystemLibrary.PrintString` "Dialogue ended")
  (`self.K2_DestroyActor`))

(event `CreateWidget`
  (`/Engine/EditorBlueprintResources/StandardMacros.IsValid` (`self.Widget`)
    (:`Is Valid`
      (`UserWidget.AddToViewport` (`self.Widget`) 0)
      (`WidgetBlueprintLibrary.SetInputMode_UIOnlyEx` (`GameplayStatics.GetPlayerController` 0) (`self.Widget`) "LockAlways" true))))

(fn `UserConstructionScript`
  (bind _bpc_dialoguecontainer (`self.BPC_DialogueContainer`))
  (if (`/Game/Blueprints/Dialogue/BPC_DialogueContainer.UseDialogueTable` _bpc_dialoguecontainer)
    (`/Game/Blueprints/Dialogue/BPC_DialogueContainer.FillDialogue` _bpc_dialoguecontainer)))