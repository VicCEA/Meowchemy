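; Quest-giving variant of a dialogue box Blueprint that hands out a quest when its dialogue widget is removed.
; The RemoveWidget override calls InteractWith on its QuestGiverComponent and passes the result to MyPlayerController's objective ID call.
; It then shows a LocationNotify widget reading "Quest Added" before running the parent's removal logic.
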(event `self.ReceiveBeginPlay`
  (`parent.ReceiveBeginPlay`))

(event `self.RemoveWidget`
  (bind _objectiveid (`/Game/QuestSystem/QuestGiverComponent.InteractWith` (`self.QuestGiverComponent`)))
  (bind _asmy_player_controller (cast `/Game/Blueprints/MyPlayerController` (`GameplayStatics.GetPlayerController` 0)))
  (`/Game/Blueprints/MyPlayerController.OnObjectiveIDCalled` _asmy_player_controller _objectiveid)
  (bind _returnvalue (`|CreateWidget` "/Game/QuestSystem/LocationNotify.LocationNotify_C" null "Quest Added"))
  (`UserWidget.AddToViewport` _returnvalue 0)
  (`parent.RemoveWidget`))

(fn `UserConstructionScript`
  (`parent.UserConstructionScript`))