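; BPC_DialogueContainer is a dialogue container that gathers the lines for one NPC conversation from the MeowchemyDialogue data table.
; FillDialogue loops over every row name and keeps rows whose NPCID and ConversationID both match those in its DialogueStruct.
; Each matching row's text is converted to a string and appended to the Dialogue array, which is not cleared first.
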(fn `FillDialogue`
  (bind (_npc_id _conversation_id) (break `/Game/Blueprints/Dialogue/FDialogueStruct` (`self.DialogueStruct`)))
  (bind _outrownames (`DataTableFunctionLibrary.GetDataTableRowNames` "/Game/Blueprints/Dialogue/MeowchemyDialogue_-_Sheet1.MeowchemyDialogue_-_Sheet1"))
  (for _array_element _outrownames
    (bind _returnvalue (`|GetDataTableRow` "/Game/Blueprints/Dialogue/MeowchemyDialogue_-_Sheet1.MeowchemyDialogue_-_Sheet1" _array_element)
      (:`then`
        (bind (_npc_id_2 _conversation_id_2 _line_id _dialogue) (break `/Game/Blueprints/Dialogue/FDialogueStruct` _returnvalue))
        (if (`KismetStringLibrary.EqualEqual_StrStr` _npc_id_2 _npc_id)
          (if (== _conversation_id_2 _conversation_id)
            (`KismetArrayLibrary.Array_Add` (`self.Dialogue`) (`KismetTextLibrary.Conv_TextToString` _dialogue))))))))