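; A Blueprint function library of small utility helpers for flipbook timing and direction math.
; It converts an animation frame count to a duration at a fixed 12 frames per second.
; Two helpers return normalized directions with opposite signs: the location version points from Target toward Initial, while the actor version points from Initial toward Target.
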(fn `CalculateDirectionBetweenTwoActors`
  (params (Initial :type "Actor Object Reference") (Target :type "Actor Object Reference"))
  (returns (NormalizedDirection :type "Vector Structure"))
  (return (`KismetMathLibrary.Normal` (- (`Actor.K2_GetActorLocation` Target) (`Actor.K2_GetActorLocation` Initial)))))

(fn `CalculateDirectionBetweenTwoLocations`
  (params (Initial :type "Vector Structure") (Target :type "Vector Structure"))
  (returns (NormalizedDirection :type "Vector Structure"))
  (return (`KismetMathLibrary.Normal` (- Initial Target))))

(fn `CalculateFlipbookDuration`
  (params (AnimationFrames :type "Float (double-precision)" :default 12.0))
  (returns (FlipbookDuration :type "Float (double-precision)"))
  (return (/ AnimationFrames 12.0)))