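; Player interaction component for BPZD_Character that focuses and interacts with BPI_Interact actors, often through the character's companion.
; Each tick it clears old focus, then sphere-traces along the move direction and notifies the interactable hits.
; Pressing interact triggers quest givers directly or sends the companion to other targets; releasing stops it and interacts with the last stored target.
; Both inputs are skipped while the companion has the BPC_CompanionPosses_Skill component.
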(event `self.ReceiveBeginPlay`
  (bind _asbpzd_character (cast `/Game/Paper2D/BPZD_Character` (`self.GetOwner`)))
  (set `self.As BPZD Character` _asbpzd_character))

(event `self.ReceiveTick`
  (params (DeltaSeconds :type "Float (single-precision)"))
  (bind _returnvalue (`Actor.K2_GetActorLocation` (`self.As BPZD Character`)))
  (`self.ClearFocusedObjects`)
  (bind (_outhits _returnvalue_2) (`KismetSystemLibrary.SphereTraceMulti` _returnvalue (+ _returnvalue (* (`KismetMathLibrary.Normal` (`/Game/Paper2D/BPZD_Character.MoveDirection` (`self.As BPZD Character`))) (`self.InteractionDistance`))) (`self.TraceRadius`) "TraceTypeQuery1" false (`|MakeArray` (`self.GetOwner`)) "None" true (struct :`R` 1.0 :`A` 1.0) (struct :`G` 1.0 :`A` 1.0) 1.0))
  (if _returnvalue_2
    (for _array_element _outhits
      (bind (_bblockinghit _binitialoverlap _time _distance _location _impactpoint _normal _impactnormal _physmat _hitactor) (`GameplayStatics.BreakHitResult` _array_element))
      (if (`KismetSystemLibrary.DoesImplementInterface` _hitactor "/Game/Blueprints/Interaction/BPI_Interact.BPI_Interact_C")
        (`KismetArrayLibrary.Array_Add` (`self.Hit Actors`) _hitactor)
        (message `/Game/Blueprints/Interaction/BPI_Interact.OnFocus` _hitactor)))))

(event `EnhancedInput|/Game/Input/IA_Interact`
  (params (ActionValue :type Boolean) (ElapsedSeconds :type "Float (double-precision)") (TriggeredSeconds :type "Float (double-precision)") (InputAction :type "InputAction Object Reference" :default "/Game/Input/IA_Interact.IA_Interact"))
  (bind _returnvalue (`self.CheckCompanionSkill`))
  (bind _interactactor (`self.InteractActor`))
  (:`Started`
    (if (not _returnvalue)
      (for _array_element (`self.Hit Actors`)
        (set `self.InteractActor` _array_element)
        (`/Engine/EditorBlueprintResources/StandardMacros.IsValid` (`Actor.GetComponentByClass` _array_element "/Game/QuestSystem/QuestGiverComponent.QuestGiverComponent_C")
          (:`Is Valid`
            (message `/Game/Blueprints/Interaction/BPI_Interact.Interact` _array_element))
          (:`Is Not Valid`
            (`/Game/Blueprints/AI/Companion/BPZD_Companion.GoToLocation` (`/Game/Paper2D/BPZD_Character.CompanionRef` (`self.As BPZD Character`)) (`Actor.K2_GetActorLocation` _array_element) "/Game/Blueprints/Abilities/Companion/BPC_CompanionPosses.BPC_CompanionPosses_C"))))))
  (:`Completed`
    (if (not _returnvalue)
      (`/Game/Blueprints/AI/Companion/BPZD_Companion.StopDirected` (`/Game/Paper2D/BPZD_Character.CompanionRef` (`self.As BPZD Character`)))
      (if (not (`Actor.IsActorBeingDestroyed` _interactactor))
        (message `/Game/Blueprints/Interaction/BPI_Interact.Interact` _interactactor)))))

(fn `CheckCompanionSkill`
  (returns (ReturnValue :type Boolean))
  (return (`KismetSystemLibrary.IsValid` (`Actor.GetComponentByClass` (`/Game/Paper2D/BPZD_Character.CompanionRef` (`self.As BPZD Character`)) "/Game/Blueprints/Abilities/Companion/BPC_CompanionPosses_Skill.BPC_CompanionPosses_Skill_C"))))

(fn `ClearFocusedObjects`
  (for _array_element (`self.Hit Actors`)
    (message `/Game/Blueprints/Interaction/BPI_Interact.OnFocusEnd` _array_element))
  (`KismetArrayLibrary.Array_Clear` (`self.Hit Actors`)))

(fn `Interact`
  (return))

(fn `InteractWithObjects`
  (for _array_element (`self.Hit Actors`)
    (message `/Game/Blueprints/Interaction/BPI_Interact.Interact` _array_element)))